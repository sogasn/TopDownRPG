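; Inventory component that stores item stacks and tracks money, carried weight, buying and selling.
; Adding routes one item type into money and others into new or partly filled same-class stacks, recursively re-adding overflow beyond max quantity.
; Purchases and sales scale prices by trade-difficulty multipliers, updating money, items and weight.
; It also refreshes item data from class defaults and toggles the inventory panel widget, passing an optional container.
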(fn `Add Money`
  (params (`Item To Add` :type "/Game/Blueprints/Inventory/Structures/ST_Slot Structure"))
  (set `self.Money` (+ (`self.Money`) `Item To Add_Quantity_8_3921FCB747438F84BE78A291CC557E27`))
  (return))

(fn `Add To Inventory`
  (params (`Item To Add` :type "/Game/Blueprints/Inventory/Structures/ST_Slot Structure"))
  (bind ((`IsStakable_29_937020CB4C93E9EEF5F038A185FA4A9A` _isstakable) (`ItemType_18_4C884E6F4321BC5E70DF60ADCF90B142` _itemtype)) (break `/Game/Blueprints/Inventory/Structures/ST_Item` `Item To Add_Item_5_8A5B53FA4EAA5A9A685C709977B0DB94`))
  (if (`|EnumInequality` _itemtype "NewEnumerator5")
    (if _isstakable
      (bind _index (`self.Check Stack Fulfillment` (`local.Item To Add`))
        (:`Add To Stack`
          (`self.Add To Stack` (`local.Item To Add`) _index))
        (:`Create New Stack`
          (`self.Create Stack` (`local.Item To Add`) :!label _label)))
      (else
        (goto _label)))
    (`self.Add Weight` (`local.Item To Add`))
    (return)
    (else
      (`self.Add Money` (`local.Item To Add`))
      (return))))

(fn `Add To Stack`
  (params (`Item To Add` :type "/Game/Blueprints/Inventory/Structures/ST_Slot Structure") (Index :type Integer))
  (locals (Quantity :type Integer))
  (bind _item_to_add_item (break `/Game/Blueprints/Inventory/Structures/ST_Slot` (`local.Item To Add`)))
  (bind _item_to_add_item_2 (break `/Game/Blueprints/Inventory/Structures/ST_Slot` (`local.Item To Add`)))
  (bind _item_to_add_item_3 (break `/Game/Blueprints/Inventory/Structures/ST_Slot` (`local.Item To Add`)))
  (bind ((`MaxQuantity_13_811DBC43489352CF7D5D1A93D468AF14` _maxquantity)) (break `/Game/Blueprints/Inventory/Structures/ST_Item` _item_to_add_item))
  (bind (_output_item _output_quantity) (break `/Game/Blueprints/Inventory/Structures/ST_Slot` (`|GetArrayItem` (`self.Inventory`) Index)))
  (bind _returnvalue (+ `Item To Add_Quantity_8_3921FCB747438F84BE78A291CC557E27` _output_quantity))
  (set `local.Quantity` _returnvalue)
  (if (> _returnvalue (`.MaxQuantity_13_811DBC43489352CF7D5D1A93D468AF14` (break `/Game/Blueprints/Inventory/Structures/ST_Item` _output_item)))
    ;[1 1 1] New Stack
    (`KismetArrayLibrary.Array_Set` (`self.Inventory`) (`local.Index`) (make `/Game/Blueprints/Inventory/Structures/ST_Slot` _item_to_add_item _maxquantity))
    (`self.Add To Inventory` (make `/Game/Blueprints/Inventory/Structures/ST_Slot` _item_to_add_item_3 (- (`local.Quantity`) _maxquantity)))
    (return)
    (else
      ;[1 1 1] Stack Can Fulfull New Item With Existing
      (`KismetArrayLibrary.Array_Set` (`self.Inventory`) (`local.Index`) (make `/Game/Blueprints/Inventory/Structures/ST_Slot` _item_to_add_item_2 (`local.Quantity`)))
      (return))))

(fn `Add Weight`
  (params (`Item To Add` :type "/Game/Blueprints/Inventory/Structures/ST_Slot Structure"))
  (bind ((`Weight_8_9EBDB6934A0707976A99D18B2C4AF6F2` _weight) (`IsStakable_29_937020CB4C93E9EEF5F038A185FA4A9A` _isstakable)) (break `/Game/Blueprints/Inventory/Structures/ST_Item` `Item To Add_Item_5_8A5B53FA4EAA5A9A685C709977B0DB94`))
  (if _isstakable
    (set `self.Weight` (+ (`self.Weight`) (* _weight `Item To Add_Quantity_8_3921FCB747438F84BE78A291CC557E27`)))
    (return)
    (else
      (set `self.Weight` (+ _weight (`self.Weight`)))
      (return))))

(fn `Check Weight`
  (params (`Item To Add` :type "/Game/Blueprints/Inventory/Structures/ST_Item Structure"))
  (returns (ReturnValue :type Boolean))
  (return (> (`.Weight_8_9EBDB6934A0707976A99D18B2C4AF6F2` (break `/Game/Blueprints/Inventory/Structures/ST_Item` `Item To Add`)) (`self.Weight`))))

(fn `Create Stack`
  (params (`Item To Add` :type "/Game/Blueprints/Inventory/Structures/ST_Slot Structure"))
  (`KismetArrayLibrary.Array_Set` (`self.Inventory`) (+ (`KismetArrayLibrary.Array_LastIndex` (`self.Inventory`)) 1) (`local.Item To Add`) true)
  (return))

(fn `Prepare Inventory`
  (for (_array_element _array_index) (`self.Inventory`)
    (bind (_name _thumbnail _description _price _weight _isstakable _maxquantity _itemtype _class) (break `/Game/Blueprints/Inventory/Structures/ST_Item` (break `/Game/Blueprints/Inventory/Structures/ST_Slot` _array_element)))
    (if (`KismetSystemLibrary.IsValidClass` _class)
      (`KismetArrayLibrary.Array_Set` (`self.Inventory`) _array_index (make `/Game/Blueprints/Inventory/Structures/ST_Slot` (defaults `Object` _class) (`.Quantity_8_3921FCB747438F84BE78A291CC557E27` (break `/Game/Blueprints/Inventory/Structures/ST_Slot` _array_element)))))))

(fn `Purchase Item`
  (params (`Item To Purchase` :type "/Game/Blueprints/Inventory/Structures/ST_Slot Structure"))
  (returns (`Is Succes?` :type Boolean))
  (locals (`Total Price` :type Integer))
  (bind ((`Price_21_0C7D4A8F401CC92B668F23A9E29ABE31` _price) (`IsStakable_29_937020CB4C93E9EEF5F038A185FA4A9A` _isstakable)) (break `/Game/Blueprints/Inventory/Structures/ST_Item` `Item To Purchase_Item_5_8A5B53FA4EAA5A9A685C709977B0DB94`))
  (if _isstakable
    (set `local.Total Price` (`KismetMathLibrary.FTrunc` (* (* _price `Item To Purchase_Quantity_8_3921FCB747438F84BE78A291CC557E27`) (`self.Trade Difficulty For Bying`))))
    (else
      (set `local.Total Price` (`KismetMathLibrary.FTrunc` (* _price (`self.Trade Difficulty For Bying`))))))
  (if (>= (- (`self.Money`) (`local.Total Price`)) 0)
    (set `self.Money` (- (`self.Money`) (`local.Total Price`)))
    (`self.Add To Inventory` (`local.Item To Purchase`))
    (return true)
    (else
      (return false))))

(fn `Remove Index Fron Inventory`
  (params (Index :type Integer))
  (`self.Remove Weight` (`|GetArrayItem` (`self.Inventory`) Index))
  (`KismetArrayLibrary.Array_Remove` (`self.Inventory`) Index)
  (return))

(fn `Remove Item From Inventory`
  (params (`Item To Remove` :type "/Game/Blueprints/Inventory/Structures/ST_Slot Structure"))
  (`self.Remove Index Fron Inventory` (`KismetArrayLibrary.Array_Find` (`self.Inventory`) `Item To Remove`))
  (return))

(fn `Remove Weight`
  (params (Item :type "/Game/Blueprints/Inventory/Structures/ST_Slot Structure"))
  (locals (`Weight To Remove` :type "Float (double-precision)"))
  (bind ((`Weight_8_9EBDB6934A0707976A99D18B2C4AF6F2` _weight) (`IsStakable_29_937020CB4C93E9EEF5F038A185FA4A9A` _isstakable)) (break `/Game/Blueprints/Inventory/Structures/ST_Item` Item_Item_5_8A5B53FA4EAA5A9A685C709977B0DB94))
  (if _isstakable
    (set `local.Weight To Remove` (* _weight Item_Quantity_8_3921FCB747438F84BE78A291CC557E27))
    (else
      (set `local.Weight To Remove` _weight)))
  (set `self.Weight` (- (`self.Weight`) (`local.Weight To Remove`)))
  (return))

(fn `Sell Item`
  (params (`Item To Sell` :type "/Game/Blueprints/Inventory/Structures/ST_Slot Structure"))
  (locals (`Total Sell Price` :type Integer))
  (bind ((`Price_21_0C7D4A8F401CC92B668F23A9E29ABE31` _price) (`IsStakable_29_937020CB4C93E9EEF5F038A185FA4A9A` _isstakable)) (break `/Game/Blueprints/Inventory/Structures/ST_Item` `Item To Sell_Item_5_8A5B53FA4EAA5A9A685C709977B0DB94`))
  (if _isstakable
    (bind _output_get (set `local.Total Sell Price` (`KismetMathLibrary.FTrunc` (* (* _price `Item To Sell_Quantity_8_3921FCB747438F84BE78A291CC557E27`) (`self.Trade Difficulty For Selling`)))))
    (else
      (set `local.Total Sell Price` (`KismetMathLibrary.FTrunc` (* _price (`self.Trade Difficulty For Selling`))))))
  (set `self.Money` (+ _output_get (`self.Money`)))
  (`self.Remove Item From Inventory` (`local.Item To Sell`))
  (return))

(fn `Toggle Inventory`
  (params (Container :type "/Game/Blueprints/Inventory/AC_Inventory Object Reference"))
  (`self.Inventory Panel`
    (:`then`
      (`Widget.RemoveFromParent` (`self.Inventory Panel`))
      (set `self.Inventory Panel` null)
      (return))
    (:`else`
      (bind _as_player (`/Game/Libraries/BlueprintFunctionLibrary.Cast To Player` 0))
      (`/Game/Blueprints/PlayerCamera/BP_PlayerCamera.Toggle Active Widgets` _as_player)
      (bind _returnvalue (`|CreateWidget` "/Game/HUD/Inventory/UMG_InventoryPanel.UMG_InventoryPanel_C" null self (`local.Container`)))
      (bind _output_get (set `self.Inventory Panel` _returnvalue))
      (`UserWidget.AddToPlayerScreen` _output_get 0)
      (return))))