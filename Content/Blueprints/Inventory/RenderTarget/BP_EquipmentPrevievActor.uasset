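; Preview actor for the inventory that displays equipped items on a skeletal mesh, apparently for render target capture.
; On BeginPlay it spawns the initial equipment below the origin, snaps each piece to its socket on the mesh and tracks it in an Equipment array.
; EquipItem does the same for a given class.
; UnequipItem finds the first tracked actor of the given class, removes it and destroys it.
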(event `self.ReceiveBeginPlay`
  ;[1 1 1] Initial Setup
  (for _array_element (`self.Initial Equipment`)
    (bind _returnvalue (`|SpawnActorFromClass` (`GameplayStatics.GetObjectClass` _array_element) (`KismetMathLibrary.MakeTransform` (0.0 0.0 -1050.0)) "Undefined" "OverrideRootScale" null null))
    (`KismetArrayLibrary.Array_AddUnique` (`self.Equipment`) _returnvalue)
    (`self.K2_AttachToComponent` _returnvalue (`self.SkeletalMesh`) (`/Game/Blueprints/Pickables/BP_PickableItem_Base.Socket To Attach` _array_element) "SnapToTarget" "SnapToTarget" "KeepWorld" true)))

(fn `Equip Item`
  (params (Class :type "/Game/Blueprints/Pickables/BP_PickableItem_Base Class Reference"))
  (bind _returnvalue (`|SpawnActorFromClass` Class (`KismetMathLibrary.MakeTransform` (0.0 0.0 -11000.0)) "Undefined" "OverrideRootScale" null null))
  (`self.K2_AttachToComponent` _returnvalue (`self.SkeletalMesh`) (`/Game/Blueprints/Pickables/BP_PickableItem_Base.Socket To Attach` _returnvalue) "SnapToTarget" "SnapToTarget" "KeepWorld" true)
  (`KismetArrayLibrary.Array_AddUnique` (`self.Equipment`) _returnvalue)
  (return))

(fn `Unequip Item`
  (params (`Class To Remove` :type "/Game/Blueprints/Pickables/BP_PickableItem_Base Class Reference"))
  (locals (`Item To Remove` :type "/Game/Blueprints/Pickables/BP_PickableItem_Base Object Reference"))
  (for _array_element (`self.Equipment`)
    (if (== (`GameplayStatics.GetObjectClass` _array_element) (`local.Class To Remove`))
      (set `local.Item To Remove` _array_element)
      (break)))
  (bind _item_to_remove (`local.Item To Remove`)
    (:`then`
      (`KismetArrayLibrary.Array_RemoveItem` (`self.Equipment`) _item_to_remove)
      (`self.K2_DestroyActor` _item_to_remove)
      (return))
    (:`else`
      (return))))

(fn `UserConstructionScript`)