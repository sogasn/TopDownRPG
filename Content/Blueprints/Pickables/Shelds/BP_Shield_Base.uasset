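; BP_Shield_Base is the base Blueprint for equippable shields that change a character's armor and agility.
; On use, it checks the character's equipped item of one type and unuses it if it is a two-handed weapon, then runs the parent logic and applies ArmorClass and AgilityPenalty to CharacterStats.
; On unuse, it removes those stat effects before calling the parent unuse.
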(fn `Unuse Item`
  (params (`Character To Unuse` :type "/Game/Blueprints/AI/Base/BP_AICharacter_Base Object Reference"))
  ;[1 1 1] Remove Effects From Armor Before Destroying Shield
  (`/Game/Blueprints/Stats/AC_CharacterStats.Remove Armor Clothes` (`/Game/Blueprints/AI/Base/BP_AICharacter_Base.Character Stats` (`local.Character To Unuse`)) (`self.Armor Class`) (`self.Agility Penalty`))
  (`parent.Unuse Item` `Character To Unuse`)
  (return))

(fn `Use Item`
  (params (`Character To Use` :type "/Game/Blueprints/AI/Base/BP_AICharacter_Base Object Reference"))
  ;[1 1 1] If Character Has Two Handed Weapon Equipped, unequip Item
  (bind _return_value (`/Game/Blueprints/AI/Base/BP_AICharacter_Base.Get Equipment Item By Type` `Character To Use` "NewEnumerator1"))
  (if (not (not (`KismetSystemLibrary.IsValid` _return_value)))
    (bind _asbp_weapon_base (cast `/Game/Blueprints/Pickables/Weapons/BP_Weapon_Base` _return_value))
    (if (not (not (`|EnumEquality` (`/Game/Blueprints/Pickables/Weapons/BP_Weapon_Base.Weapon Type` _asbp_weapon_base) "NewEnumerator2")))
      (`self.Unuse Item` _return_value `Character To Use`)))
  (`parent.Use Item` `Character To Use`)
  ;[1 1 1] Add Armor Class And Agility Penalty
  (`/Game/Blueprints/Stats/AC_CharacterStats.Add Armor Clothes` (`/Game/Blueprints/AI/Base/BP_AICharacter_Base.Character Stats` `Character To Use`) (`self.Armor Class`) (`self.Agility Penalty`))
  (return))

(fn `UserConstructionScript`
  (`parent.UserConstructionScript`))