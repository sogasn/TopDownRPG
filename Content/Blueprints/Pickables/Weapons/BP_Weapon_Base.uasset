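; Base Blueprint for pickable weapons, built on a parent class that provides the item-use behavior.
; UseItem runs the parent logic, then checks the WeaponTypeRange enum and sets IsRangedWeaponEquipped on the using character when it matches the second enumerator.
; The flag is only ever set to true here; other range types leave it untouched.
; BeginPlay and the construction script only call their parents.
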(event `self.ReceiveBeginPlay`
  (`parent.ReceiveBeginPlay`))

(fn `Use Item`
  (params (`Character To Use` :type "/Game/Blueprints/AI/BP_AICharacter_Base Object Reference"))
  (`parent.Use Item` `Character To Use`)
  (if (`|EnumEquality` (`self.Weapon Type Range`) "NewEnumerator1")
    (set `/Game/Blueprints/AI/BP_AICharacter_Base.Is Ranged Weapon Equipped?` true (`local.Character To Use`))
    (return)
    (else
      (return))))

(fn `UserConstructionScript`
  (`parent.UserConstructionScript`))