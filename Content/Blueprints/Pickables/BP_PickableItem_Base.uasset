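; Base actor for pickable, equippable items that go into the party inventory when a character with a specific player attitude interacts.
; Hovering or a toggle event shows a name widget, kept rotated to the player and scaled by camera arm length on a looping timer.
; UseItem, also run at BeginPlay for a valid Character, swaps out same-type equipment and attaches to a mesh socket.
; UnuseItem unequips, returning all but one item type to inventory and destroying the actor.
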(event `/Game/Libraries/BPI_Interact.Toggle Widget Name`
  (params (`Is Displaying?` :type Boolean))
  ;[1 1 1] Toggle Widget Name
  (if `Is Displaying?`
    (`self.Set Object Name Visibility` :!label _label)
    (`KismetSystemLibrary.K2_SetTimer` null "Set Object Name Visibility" 0.01 true)
    (else
      (`self.Hide Object Name` :!label _label_2))))

(event `self.ReceiveActorBeginCursorOver`
  ;[1 1 1] Toggle Widget Name
  (goto _label))

(event `self.ReceiveActorEndCursorOver`
  ;[1 1 1] Toggle Widget Name
  (if (not (stale `/Game/Libraries/BPI_Interact.Toggle Widget Name` `Is Displaying?`))
    (goto _label_2)))

(event `/Game/Libraries/BPI_Interact.Interact`
  (params (Interacter :type "Actor Object Reference"))
  ;[1 1 1] Interaction
  (bind _asbp_aicharacter_base (cast `/Game/Blueprints/AI/BP_AICharacter_Base` Interacter))
  (if (`|EnumEquality` (`/Game/Blueprints/AI/BP_AICharacter_Base.Attitude Towards Player` _asbp_aicharacter_base) "NewEnumerator3")
    (bind _as_player (`/Game/Libraries/BlueprintFunctionLibrary.Cast To Player` 0))
    (`/Game/Blueprints/Inventory/AC_Inventory.Add To Inventory` (`/Game/Blueprints/PlayerCamera/BP_PlayerCamera.Party Inventory` _as_player) (make `/Game/Blueprints/Inventory/Structures/ST_Slot` (`self.Item`) 1))
    (`self.K2_DestroyActor`)))

(event `self.ReceiveBeginPlay`
  ;[1 1 1] Initial Setup
  (bind _asumg_object_name (cast `/Game/HUD/UMG_ObjectName` (`WidgetComponent.GetWidget` (`self.Widget`))))
  (set `self.Object Name` _asumg_object_name)
  (bind _as_player (`/Game/Libraries/BlueprintFunctionLibrary.Cast To Player` 0))
  (set `self.Player Cast` _as_player)
  (bind _character (`self.Character`)
    (:`then`
      (`self.Use Item` self _character))
    (:`else`)))

(fn `Hide Object Name`
  (`KismetSystemLibrary.K2_ClearTimer` null "Set Object Name Visibility")
  (`SceneComponent.SetVisibility` (`self.Widget`) false false))

(fn `Set Object Name Visibility`
  (bind (_returnvalue_roll _returnvalue_pitch _returnvalue_yaw) (`KismetMathLibrary.BreakRotator` (`self.K2_GetActorRotation` (`self.Player Cast`))))
  (if (not (`self.Is Equipped?`))
    (`SceneComponent.SetVisibility` (`self.Widget`) true false)
    (`SceneComponent.K2_SetRelativeRotation` (`self.Widget`) (`KismetMathLibrary.MakeRotator` (- _returnvalue_roll 180.0) (- _returnvalue_pitch -125.0) _returnvalue_yaw) false false)
    (set `/Game/HUD/UMG_ObjectName.Name` (`.Name_6_9780479243081C6B8006CFA806C9EF9D` (break `/Game/Blueprints/Inventory/Structures/ST_Item` (`self.Item`))) (`self.Object Name`))
    (`SceneComponent.SetRelativeScale3D` (`self.Widget`) (`KismetMathLibrary.Conv_DoubleToVector` (/ (`SpringArmComponent.TargetArmLength` (`/Game/Blueprints/PlayerCamera/BP_PlayerCamera.SpringArm` (`self.Player Cast`))) (`self.Scale Divider`))))
    (return)
    (else
      (return))))

(fn `Unuse Item`
  (params (`Character To Unuse` :type "/Game/Blueprints/AI/BP_AICharacter_Base Object Reference"))
  (`/Game/Blueprints/AI/BP_AICharacter_Base.Remove From Equipment` `Character To Unuse` self)
  (if (`|EnumInequality` (`.ItemType_18_4C884E6F4321BC5E70DF60ADCF90B142` (break `/Game/Blueprints/Inventory/Structures/ST_Item` (`self.Item`))) "NewEnumerator6")
    (`/Game/Blueprints/Inventory/AC_Inventory.Add To Inventory` (`/Game/Blueprints/PlayerCamera/BP_PlayerCamera.Party Inventory` (`self.Player Cast`)) (make `/Game/Blueprints/Inventory/Structures/ST_Slot` (`self.Item`) 1))
    (`/Game/HUD/Equipment/UMG_EquipmentPanel.Refresh Inventory` (`/Game/Blueprints/PlayerCamera/BP_PlayerCamera.Equipment Panel` (`self.Player Cast`)))
    (`self.K2_DestroyActor` self)
    (return)
    (else
      (return))))

(fn `Use Item`
  (params (`Character To Use` :type "/Game/Blueprints/AI/BP_AICharacter_Base Object Reference"))
  (locals (`Old Item` :type "/Game/Blueprints/Pickables/BP_PickableItem_Base Object Reference"))
  ;[1 1 1] Check For Item Of Same Type
  (for _array_element (`/Game/Blueprints/AI/BP_AICharacter_Base.Equipment` `Character To Use`)
    (if (`|EnumEquality` (`.ItemType_18_4C884E6F4321BC5E70DF60ADCF90B142` (break `/Game/Blueprints/Inventory/Structures/ST_Item` (`/Game/Blueprints/Pickables/BP_PickableItem_Base.Item` _array_element))) (`.ItemType_18_4C884E6F4321BC5E70DF60ADCF90B142` (break `/Game/Blueprints/Inventory/Structures/ST_Item` (`self.Item`))))
      (set `local.Old Item` _array_element)))
  ;[1 1 1] Unequip Item If Same Exist
  (bind _old_item (`local.Old Item`)
    (:`then`
      (`self.Unuse Item` _old_item (`local.Character To Use`)))
    (:`else`
      _))
  (`self.K2_AttachToComponent` self (`Character.Mesh` (`local.Character To Use`)) (`self.Socket To Attach`) "SnapToTarget" "SnapToTarget" "KeepWorld" true)
  (set `self.Is Equipped?` true)
  (`PrimitiveComponent.SetCollisionEnabled` (`self.Box`) "NoCollision")
  (`/Game/Blueprints/AI/BP_AICharacter_Base.Add To Equipment` (`local.Character To Use`) self)
  (return))

(fn `UserConstructionScript`)