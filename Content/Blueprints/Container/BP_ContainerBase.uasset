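; Base actor for interactable containers that open their inventory through the player's party inventory.
; BeginPlay fills the inventory, caches player and name widget, and detects an attached BP_Lock.
; Interact attempts to break a valid lock, otherwise opens the inventory; successful lockpicking also opens it.
; Cursor hover or toggle event shows a name/lock-integrity widget, using a looping timer to orient it by player rotation and scale it by camera arm length.
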(event `/Game/Libraries/BPI_Interact.Toggle Widget Name`
  (params (`Is Displaying?` :type Boolean))
  ;[1 1 1] Toggle Widget Name
  (if `Is Displaying?`
    (`self.Set Object Name Visibility` :!label _label)
    (`KismetSystemLibrary.K2_SetTimer` null "Set Object Name Visibility" 0.01 true)
    (else
      (`self.Hide Object Name` :!label _label_2))))

(event `self.ReceiveActorBeginCursorOver`
  ;[1 1 1] Toggle Widget Name
  (goto _label))

(event `self.ReceiveActorEndCursorOver`
  ;[1 1 1] Toggle Widget Name
  (if (not (stale `/Game/Libraries/BPI_Interact.Toggle Widget Name` `Is Displaying?`))
    (goto _label_2)))

(event `self.ReceiveBeginPlay`
  ;[1 1 1] Begin Play
  (set `/Game/Blueprints/Inventory/AC_Inventory.Inventory` (`self.Inventory Content`) (`self.Inventory`))
  (bind _asumg_object_name (cast `/Game/HUD/UMG_ObjectName` (`WidgetComponent.GetWidget` (`self.Widget`))))
  (set `self.Object Name` _asumg_object_name)
  (bind _as_player (`/Game/Libraries/BlueprintFunctionLibrary.Cast To Player` 0))
  (set `self.Player Cast` _as_player)
  (for _array_element (`self.GetAttachedActors` true)
    (bind _asbp_lock (cast `/Game/Blueprints/Lock/BP_Lock` _array_element))
    (set `self.Lock` _asbp_lock)
    (break)))

(event `/Game/Libraries/BPI_Interact.Interact`
  (params (Interacter :type "Actor Object Reference"))
  ;[1 1 1] Interaction
  (bind _lock (`self.Lock`)
    (:`then`
      (bind _asbp_aicharacter_base (cast `/Game/Blueprints/AI/Base/BP_AICharacter_Base` Interacter))
      (`KismetSystemLibrary.Delay` 0.2)
      (`/Game/Blueprints/Lock/BP_Lock.Break Lock` _lock _asbp_aicharacter_base))
    (:`else`
      (`KismetSystemLibrary.Delay` 0.2)
      (`/Game/Blueprints/Inventory/AC_Inventory.Toggle Inventory` (`/Game/Blueprints/PlayerCamera/BP_PlayerCamera.Party Inventory` (`self.Player Cast`)) (`self.Inventory`)))))

(fn `Hide Object Name`
  (`KismetSystemLibrary.K2_ClearTimer` null "Set Object Name Visibility")
  (`SceneComponent.SetVisibility` (`self.Widget`) false false))

(fn `Lockpicking Result`
  (params (`Input Value` :type Boolean))
  (if `Input Value`
    (`/Game/Blueprints/Inventory/AC_Inventory.Toggle Inventory` (`/Game/Blueprints/PlayerCamera/BP_PlayerCamera.Party Inventory` (`self.Player Cast`)) (`self.Inventory`))))

(fn `Set Object Name Visibility`
  (locals (NewLocalVar_0 :type "Float (double-precision)"))
  (bind _object_name (`self.Object Name`))
  (bind (_returnvalue_roll _returnvalue_pitch _returnvalue_yaw) (`KismetMathLibrary.BreakRotator` (`self.K2_GetActorRotation` (`self.Player Cast`))))
  (`SceneComponent.SetVisibility` (`self.Widget`) true false)
  (`SceneComponent.K2_SetRelativeRotation` (`self.Widget`) (`KismetMathLibrary.MakeRotator` (- _returnvalue_roll 180.0) (- _returnvalue_pitch -125.0) _returnvalue_yaw) false false)
  (set `/Game/HUD/UMG_ObjectName.Name` (`self.Inventory Name`) _object_name)
  (bind _lock (`self.Lock`)
    (:`then`
      (set `/Game/HUD/UMG_ObjectName.Has HP?` true _object_name)
      (set `/Game/HUD/UMG_ObjectName.Object Health` (`KismetMathLibrary.Conv_IntToDouble` (`/Game/Blueprints/Lock/BP_Lock.Lock Integrity` _lock)) _object_name)
      (set `/Game/HUD/UMG_ObjectName.Object Health Max` (`KismetMathLibrary.Conv_IntToDouble` (`/Game/Blueprints/Lock/BP_Lock.Lock Max Integrity` _lock)) _object_name))
    (:`else`
      _))
  (`SceneComponent.SetRelativeScale3D` (`self.Widget`) (`KismetMathLibrary.Conv_DoubleToVector` (/ (`SpringArmComponent.TargetArmLength` (`/Game/Blueprints/PlayerCamera/BP_PlayerCamera.SpringArm` (`self.Player Cast`))) (`self.Scale Divider`))))
  (return))

(fn `UserConstructionScript`)