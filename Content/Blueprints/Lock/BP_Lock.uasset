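; BP_Lock is a lock actor that resolves lockpicking attempts on the container it is attached to.
; On BeginPlay it caches its attach parent as a BP_ContainerBase.
; BreakLock adds the interacter's RNG dice throw to their Trickery and passes success to the container only if the total exceeds LockDifficulty, so ties fail.
; A helper snaps the lock to the parent's location, while DestroyLock is an empty stub.
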(event `self.ReceiveBeginPlay`
  (bind _asbp_container_base (cast `/Game/Blueprints/Container/BP_ContainerBase` (`self.GetAttachParentActor`)))
  (set `self.Attached Container` _asbp_container_base))

(fn `Break Lock`
  (params (Interacter :type "/Game/Blueprints/AI/Base/BP_AICharacter_Base Object Reference"))
  (bind _character_stats (`/Game/Blueprints/AI/Base/BP_AICharacter_Base.Character Stats` Interacter))
  (bind _attached_container (`self.Attached Container`))
  (bind _rng_value (`/Game/Blueprints/Stats/AC_CharacterStats.Throw RNG DICE` _character_stats))
  (`/Engine/EditorBlueprintResources/StandardMacros.CompareInt` (+ _rng_value (`/Game/Blueprints/Stats/AC_CharacterStats.Trickery` _character_stats)) (`self.Lock Difficulty`)
    (:`>`
      (`/Game/Blueprints/Container/BP_ContainerBase.Lockpicking Result` _attached_container true))
    (:`==`
      (`/Game/Blueprints/Container/BP_ContainerBase.Lockpicking Result` _attached_container false :!label _label))
    (:`<`
      (goto _label)))
  (return))

(fn `Destroy Lock`)

(fn `Set Parent World Location`
  (`self.K2_SetActorLocation` (`self.K2_GetActorLocation` (`self.GetAttachParentActor`)))
  (return))

(fn `UserConstructionScript`)