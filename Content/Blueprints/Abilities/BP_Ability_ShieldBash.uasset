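; Shield Bash ability that lets a shield-wearing character knock back and damage a target within its radius.
; It overrides the parent ability's cast check, cast and target-effect functions.
; On a hit, when the caster's characteristic modifier plus skill exceeds the defence value, it pushes and damages the target; otherwise the target plays a deflect animation.
; Defence is currently zero, as the target's dice roll plus difficulty is left unused.
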(fn `Affect Target`
  (params (Target :type "/Game/Blueprints/AI/Base/BP_AICharacter_Base Object Reference"))
  (locals (`Ability Attack Value` :type Integer) (`Defence Value` :type Integer))
  (bind _character_stats (`/Game/Blueprints/AI/Base/BP_AICharacter_Base.Character Stats` (`self.Character`)))
  (`parent.Affect Target` Target)
  ;[1 1 1] Calculate Hit Chance
  (set `local.Ability Attack Value` (+ (`/Game/Blueprints/Stats/AC_CharacterStats.Get Characteristic Modifier On Enum` _character_stats "NewEnumerator0") (`/Game/Blueprints/Stats/AC_CharacterStats.Get Skill Value` _character_stats "NewEnumerator0")))
  (bind _rng_value (`/Game/Blueprints/Stats/AC_CharacterStats.Throw RNG DICE` (`/Game/Blueprints/AI/Base/BP_AICharacter_Base.Character Stats` (`local.Target`))))
  (bind _output_get (set `local.Defence Value` 0))
  (`/Engine/EditorBlueprintResources/StandardMacros.CompareInt` (`local.Ability Attack Value`) _output_get
    (:`>`
      (`/Game/Blueprints/AI/Base/BP_AICharacter_Base.Event Push Character Back` (`local.Target`) (`self.Character`) :!pinned true) ; Push Character Back
      (`/Game/Blueprints/AI/Base/BP_AICharacter_Base.Event Take Ability Damage` (`local.Target`) (+ (/ (`/Game/Blueprints/Stats/AC_CharacterStats.Get Characteristic Modifier On Enum` (`/Game/Blueprints/AI/Base/BP_AICharacter_Base.Character Stats` (`self.Character`)) "NewEnumerator0") 4) (`self.Damage Base`)) :!pinned true) ; Damage Ability Target
      (return))
    (:`==`
      _)
    (:`<`
      _))
  (`/Game/Blueprints/AI/Base/BP_AICharacter_Base.Deflect Animation` (`local.Target`))
  (return))

(fn `Can Cast Ability?`
  (returns (`Return Value` :type Boolean))
  (return (`/Game/Blueprints/Stats/AC_CharacterStats.Is Vearing Shield` (`/Game/Blueprints/AI/Base/BP_AICharacter_Base.Character Stats` (`self.Character`)))) ; Character can only cast ability if wearing shield
)

(fn `Cast Ability`
  (params (`Ability Target` :type "/Game/Blueprints/AI/Base/BP_AICharacter_Base Object Reference"))
  (if (<= (`self.GetDistanceTo` `Ability Target` (`self.Character`)) (`self.Radius`))
    (`parent.Cast Ability` (`local.Ability Target`))))

(fn `UserConstructionScript`
  (`parent.UserConstructionScript`))