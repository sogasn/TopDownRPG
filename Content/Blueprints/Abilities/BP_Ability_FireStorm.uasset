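; BP_Ability_FireStorm is a Fire Storm ability that spawns a BP_FireStorm actor at the cursor cast location.
; It overrides SpawnAbilityProjectile, calling the parent first, then passing the spawned actor the owning Character, the ability difficulty, and damage the Character calculates from the base value.
; The event graph holds only disabled or empty stubs, so any other casting logic comes from the parent class.
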(fn `Spawn Ability Projectile`
  (params (`Ability Target` :type "/Game/Blueprints/AI/Base/BP_AICharacter_Base Object Reference"))
  (bind _character (`self.Character`))
  (`parent.Spawn Ability Projectile` `Ability Target`)
  (`|SpawnActorFromClass` "/Game/Blueprints/Abilities/SpawnActors/BP_FireStorm.BP_FireStorm_C" (`KismetMathLibrary.MakeTransform` (`self.Cursor Cast Location`)) "Undefined" "OverrideRootScale" null (`/Game/Blueprints/AI/Base/BP_AICharacter_Base.Calculate Ability Damage` _character (`self.Damage Base`)) (`self.Ability Difficulty`) _character null))

(fn `UserConstructionScript`
  (`parent.UserConstructionScript`))