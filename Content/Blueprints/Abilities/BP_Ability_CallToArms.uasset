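; Call to Arms ability that buffs attack modifiers of characters within a radius who share the caster's hostility toward the player.
; After an animation delay, affected characters gain the effect and a render outline and are tracked in CharactersAffected.
; Duration drops per turn via StartTurnEffects, or per second via a looping timer outside fights, removing everything at zero.
; Tick prints the affected count.
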(event `self.ReceiveBeginPlay`
  (`parent.ReceiveBeginPlay`))

(event `self.Delay Before Animation`
  (params (`Ability Target` :type "/Game/Blueprints/AI/Base/BP_AICharacter_Base Object Reference"))
  ;[1 1 1] Delay Before Animation Override
  (set `self.Character Is Hostile` (`/Game/Blueprints/AI/Base/BP_AICharacter_Base.Is Character Hostile?` (`self.Character`)))
  (`KismetSystemLibrary.Delay` 0.3)
  (`self.Play Ability Animation`)
  (`KismetSystemLibrary.Delay` (`self.Animation Delay`))
  (for _array_element (`/Game/Libraries/BlueprintFunctionLibrary.Get All Characters In Range` (`self.K2_GetActorLocation` (`self.Character`)) (`self.Radius`))
    (if (== (`|EnumEquality` (`/Game/Blueprints/AI/Base/BP_AICharacter_Base.Attitude Towards Player` _array_element) "NewEnumerator1") (`self.Character Is Hostile`))
      (`self.Affect Target` _array_element)
      (`/Game/Blueprints/AI/Base/BP_AICharacter_Base.Set Render Outline` _array_element 3)
      (`KismetArrayLibrary.Array_AddUnique` (`self.Characters Affected`) _array_element)
      (`/Game/Blueprints/AI/Base/BP_AICharacter_Base.Increase Attack Modifiers` _array_element (`self.Attack Modifier Increasment`))))
  (`KismetSystemLibrary.K2_SetTimer` null "Count Seconds Remaining" 1.0 true))

(event `/Game/Blueprints/Abilities/SpawnActors/BPI_EffectPerTurn.Start Turn Effects`
  ;[1 1 1] Start Turn Effects
  (`/Engine/EditorBlueprintResources/StandardMacros.DoOnce` false :!label _label
    (:`Completed`
      (`self.Count Turns Remaining`)
      (`KismetSystemLibrary.Delay` 1.0)
      (goto _label :!via `Reset`))))

(event `self.ReceiveTick`
  (params (DeltaSeconds :type "Float (single-precision)"))
  (`KismetSystemLibrary.PrintString` (`KismetStringLibrary.Conv_IntToString` (`KismetArrayLibrary.Array_Length` (`self.Characters Affected`)))))

(fn `Affect Target`
  (params (Target :type "/Game/Blueprints/AI/Base/BP_AICharacter_Base Object Reference"))
  (`/Game/Blueprints/AI/Base/BP_AICharacter_Base.Add To Effects` Target self))

(fn `Count Seconds Remaining`
  (if (not (`/Game/Blueprints/PlayerCamera/BP_PlayerCamera.Is In Fight` (`self.Player Cast`)))
    (bind _result (`/Engine/EditorBlueprintResources/StandardMacros.DecrementInt` (`self.Number Of Turns Current`))
      (:`  `
        (if (== _result 0)
          (for _array_element (`self.Characters Affected`)
            (`/Game/Blueprints/AI/Base/BP_AICharacter_Base.Remove Effect` _array_element self)
            (`/Game/Blueprints/AI/Base/BP_AICharacter_Base.Remove Render Outline` _array_element)
            (`/Game/Blueprints/AI/Base/BP_AICharacter_Base.Remove Attack Modifiers` _array_element (`self.Attack Modifier Increasment`)))
          ;[1 1 1] Remove Affected Characters And Reset Turns
          (`self.Reset Number Of Turns`)
          (`KismetArrayLibrary.Array_Clear` (`self.Characters Affected`))
          (return))))))

(fn `Count Turns Remaining`
  (bind _result (`/Engine/EditorBlueprintResources/StandardMacros.DecrementInt` (`self.Number Of Turns Current`))
    (:`  `
      (if (== _result 0)
        (for _array_element (`self.Characters Affected`)
          (`/Game/Blueprints/AI/Base/BP_AICharacter_Base.Remove Effect` _array_element self)
          (`/Game/Blueprints/AI/Base/BP_AICharacter_Base.Remove Render Outline` _array_element)
          (`/Game/Blueprints/AI/Base/BP_AICharacter_Base.Remove Attack Modifiers` _array_element (`self.Attack Modifier Increasment`)))
        ;[1 1 1] Remove Affected Characters And Reset Turns
        (`self.Reset Number Of Turns`)
        (`KismetArrayLibrary.Array_Clear` (`self.Characters Affected`))
        (return)))))

(fn `Reset Number Of Turns`
  (set `self.Number Of Turns Current` (`self.Number Of Turns Base`))
  (`KismetSystemLibrary.K2_ClearTimer` null "Count Seconds Remaining"))

(fn `UserConstructionScript`
  (`parent.UserConstructionScript`))