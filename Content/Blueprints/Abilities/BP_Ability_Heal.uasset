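; Heal ability Blueprint that restores health to its target when a dice check succeeds.
; Affect Target runs the parent logic, then adds the target's RNG dice roll to its hit-characteristic modifier, succeeding only strictly above the ability difficulty.
; Success adds base healing plus half a skill value, with roll, modifier and skill all read from the target's CharacterStats.
; Animation is left to the parent class.
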(fn `Affect Target`
  (params (Target :type "/Game/Blueprints/AI/Base/BP_AICharacter_Base Object Reference"))
  (bind _character_stats (`/Game/Blueprints/AI/Base/BP_AICharacter_Base.Character Stats` Target))
  (`parent.Affect Target` Target)
  (bind _rng_value (`/Game/Blueprints/Stats/AC_CharacterStats.Throw RNG DICE` _character_stats))
  (`/Engine/EditorBlueprintResources/StandardMacros.CompareInt` (+ _rng_value (`/Game/Blueprints/Stats/AC_CharacterStats.Get Characteristic Modifier On Enum` _character_stats (`self.Ability Hit Characteristic`))) (`self.Ability Difficulty`)
    (:`>`
      (`/Game/Blueprints/Stats/AC_CharacterStats.Add Health` _character_stats (+ (`self.Health To Heal Base`) (/ (`/Game/Blueprints/Stats/AC_CharacterStats.Get Skill Value` _character_stats "NewEnumerator5") 2)))
      (return))
    (:`==`
      _)
    (:`<`
      _))
  (return))

(fn `Play Ability Animation`
  (`parent.Play Ability Animation`))

(fn `UserConstructionScript`
  (`parent.UserConstructionScript`))