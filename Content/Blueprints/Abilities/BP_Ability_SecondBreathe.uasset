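; Second Breathe ability for a turn-based system, which applies a heal-over-time effect to its target.
; The SpawnAbilityProjectile override calls the parent, then runs the character's hit calculation, using the base heal per turn as the difficulty.
; On success it spawns a BP_SecondBreathe effect actor at the target, with healing boosted by half a character skill value, and adds it to the target's effects.
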(fn `Spawn Ability Projectile`
  (params (`Ability Target` :type "/Game/Blueprints/AI/Base/BP_AICharacter_Base Object Reference"))
  (bind _ability_target (`local.Ability Target`))
  (`parent.Spawn Ability Projectile` `Ability Target`)
  (if (`/Game/Blueprints/AI/Base/BP_AICharacter_Base.Calculate Ability Hit` (`self.Character`) `Ability Target` (`self.Heal Per Turn Base`))
    (bind _returnvalue (`|SpawnActorFromClass` "/Game/Blueprints/Abilities/SpawnActors/BP_SecondBreathe.BP_SecondBreathe_C" (`self.GetTransform` _ability_target) "Undefined" "OverrideRootScale" null _ability_target (+ (`self.Heal Per Turn Base`) (/ (`/Game/Blueprints/Stats/AC_CharacterStats.Get Skill Value` (`/Game/Blueprints/AI/Base/BP_AICharacter_Base.Character Stats` (`self.Character`)) "NewEnumerator5") 2)) (`self.Number Of Turns`) null))
    (`/Game/Blueprints/AI/Base/BP_AICharacter_Base.Add To Effects` (`local.Ability Target`) _returnvalue)))

(fn `UserConstructionScript`
  (`parent.UserConstructionScript`))