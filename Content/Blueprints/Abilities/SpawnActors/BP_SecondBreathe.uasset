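; Spawned ability actor for Second Breathe, a heal-over-time effect that attaches to the ability target's mesh.
; Each turn-start event adds health through the target's CharacterStats and decrements the turn counter.
; A HealPerSecond variant does the same only while the player is out of a fight, though nothing in this file calls it.
; When the counter reaches zero, the FX deactivates and the actor destroys itself after a short delay.
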(event `self.ReceiveActorBeginOverlap`
  (params (OtherActor :type "Actor Object Reference"))
  (`parent.ReceiveActorBeginOverlap` OtherActor))

(event `self.ReceiveTick`
  (params (DeltaSeconds :type "Float (single-precision)"))
  (`parent.ReceiveTick` DeltaSeconds))

(event `self.ReceiveBeginPlay`
  (`parent.ReceiveBeginPlay`)
  (bind _as_player (`/Game/Libraries/BlueprintFunctionLibrary.Cast To Player` 0))
  (set `self.Player Cast` _as_player)
  (`self.K2_AttachToComponent` (`Character.Mesh` (`self.Ability Target`)) "None" "SnapToTarget" "SnapToTarget" "SnapToTarget"))

(event `Delete Actor`
  ;[1 1 1] effect finish
  (`ActorComponent.Deactivate` (`self.fx`))
  (`KismetSystemLibrary.Delay` 2.5)
  ;[1 1 1] effect delete
  (`self.K2_DestroyActor`))

(event `/Game/Blueprints/Abilities/SpawnActors/BPI_EffectPerTurn.Start Turn Effects`
  (`self.Heal Per Turn`))

(fn `Heal Per Second`
  (if (not (`/Game/Blueprints/PlayerCamera/BP_PlayerCamera.Is In Fight` (`self.Player Cast`)))
    (`/Game/Blueprints/Stats/AC_CharacterStats.Add Health` (`/Game/Blueprints/AI/Base/BP_AICharacter_Base.Character Stats` (`self.Ability Target`)) (`self.Healing Per Turn`))
    (bind _result (`/Engine/EditorBlueprintResources/StandardMacros.DecrementInt` (`self.Number Of Turns`))
      (:`  `
        (if (== _result 0)
          (`self.Delete Actor`))))))

(fn `Heal Per Turn`
  (`/Game/Blueprints/Stats/AC_CharacterStats.Add Health` (`/Game/Blueprints/AI/Base/BP_AICharacter_Base.Character Stats` (`self.Ability Target`)) (`self.Healing Per Turn`))
  (bind _result (`/Engine/EditorBlueprintResources/StandardMacros.DecrementInt` (`self.Number Of Turns`))
    (:`  `
      (if (== _result 0)
        (`self.Delete Actor`)))))

(fn `UserConstructionScript`
  (`parent.UserConstructionScript`))