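; BP_FireStorm is a spawned ability actor that deals one delayed burst of area damage at its location.
; After parent BeginPlay and a short delay, it gathers all characters within Radius.
; Its Character reference rolls CalculateAbilityHit against each target using Difficulty, and each one hit receives Damage through EventTakeAbilityDamage.
; Overlap, Tick and construction only forward to the parent class.
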(event `self.ReceiveBeginPlay`
  (`parent.ReceiveBeginPlay`)
  (`KismetSystemLibrary.Delay` 1.5)
  (for _array_element (`/Game/Libraries/BlueprintFunctionLibrary.Get All Characters In Range` (`self.K2_GetActorLocation`) (`self.Radius`))
    (if (`/Game/Blueprints/AI/Base/BP_AICharacter_Base.Calculate Ability Hit` (`self.Character`) _array_element (`self.Difficulty`))
      (`/Game/Blueprints/AI/Base/BP_AICharacter_Base.Event Take Ability Damage` _array_element (`self.Damage`)))))

(event `self.ReceiveActorBeginOverlap`
  (params (OtherActor :type "Actor Object Reference"))
  (`parent.ReceiveActorBeginOverlap` OtherActor))

(event `self.ReceiveTick`
  (params (DeltaSeconds :type "Float (single-precision)"))
  (`parent.ReceiveTick` DeltaSeconds))

(fn `UserConstructionScript`
  (`parent.UserConstructionScript`))