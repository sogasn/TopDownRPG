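; Base ability Blueprint that provides shared cooldown logic for player spells.
; Use Spell resets the cooldown counter to its base value when the ability is ready, with no spell effect of its own.
; A looping one-second timer counts the cooldown down only while the cached player is out of a fight.
; A separate fight function decrements it by one per call, with no caller in this file.
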(event `self.ReceiveBeginPlay`
  ;[1 1 1] Initial Setup
  (bind _as_player (`/Game/Libraries/BlueprintFunctionLibrary.Cast To Player` 0))
  (set `self.Player Cast` _as_player)
  (`KismetSystemLibrary.K2_SetTimer` null "Decrease Cooldown (Timer)" 1.0 true))

(fn `Decrease Cooldown (Fight)`
  (if (not (`self.Is NOT on Cooldown`))
    (`/Engine/EditorBlueprintResources/StandardMacros.DecrementInt` (`self.Cooldown Current`)
      (:`  `
        (return)))
    (else
      (return))))

(fn `Decrease Cooldown (Timer)`
  (if (not (or (`self.Is NOT on Cooldown`) (`/Game/Blueprints/PlayerCamera/BP_PlayerCamera.Is In Fight` (`self.Player Cast`)))) :!pinned true
    (`/Engine/EditorBlueprintResources/StandardMacros.DecrementInt` (`self.Cooldown Current`)
      (:`  `
        (return)))
    (else
      (return))))

(fn `Is NOT on Cooldown`
  (returns (`Return Value` :type Boolean))
  (return (== (`self.Cooldown Current`) 0)))

(fn `Set Ability On Cooldown`
  (set `self.Cooldown Current` (`self.Cooldown Base`))
  (return))

(fn `Use Spell`
  (if (`self.Is NOT on Cooldown`)
    (`self.Set Ability On Cooldown`)))

(fn `UserConstructionScript`)