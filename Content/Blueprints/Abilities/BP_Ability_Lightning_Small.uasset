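; Small lightning ability Blueprint that strikes at the cursor's cast location, built as a child of a parent ability class.
; It overrides SpawnAbilityProjectile, calls the parent version, then spawns a BP_Lightning_Small actor at that location.
; The spawned actor receives the radius, damage calculated by the character from the base damage, the owning character and the ability difficulty.
; BeginPlay and the construction script only call their parents.
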(event `self.ReceiveBeginPlay`
  (`parent.ReceiveBeginPlay`))

(fn `Spawn Ability Projectile`
  (params (`Ability Target` :type "/Game/Blueprints/AI/Base/BP_AICharacter_Base Object Reference"))
  (`parent.Spawn Ability Projectile` `Ability Target`)
  (`|SpawnActorFromClass` "/Game/Blueprints/Abilities/SpawnActors/BP_Lightning_Small.BP_Lightning_Small_C" (`KismetMathLibrary.MakeTransform` (`self.Cursor Cast Location`)) "Undefined" "OverrideRootScale" null (`self.Radius`) (`/Game/Blueprints/AI/Base/BP_AICharacter_Base.Calculate Ability Damage` (`self.Character`) (`self.Damage Base`)) (`self.Character`) (`self.Ability Difficulty`) null))

(fn `UserConstructionScript`
  (`parent.UserConstructionScript`))