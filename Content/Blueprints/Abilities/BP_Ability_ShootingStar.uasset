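; Shooting Star ability, a child Blueprint that casts a damaging ability on a target actor.
; Casting proceeds to the parent's logic only when the target is valid.
; The projectile spawn override calls the parent, then has the owning Character resolve hit and damage from the ability's difficulty and base damage.
; It spawns an actor at the target's transform, passing in that precomputed result along with the target and caster.
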(fn `Cast Ability`
  (params (`Ability Target` :type "/Game/Blueprints/AI/Base/BP_AICharacter_Base Object Reference"))
  (`/Engine/EditorBlueprintResources/StandardMacros.IsValid` `Ability Target`
    (:`Is Valid`
      (`parent.Cast Ability` `Ability Target`))))

(fn `Spawn Ability Projectile`
  (params (`Ability Target` :type "/Game/Blueprints/AI/Base/BP_AICharacter_Base Object Reference"))
  (bind _ability_target (`local.Ability Target`))
  (`parent.Spawn Ability Projectile` `Ability Target`)
  ;[1 1 1] Calculate Attack Value
  (set `self.Is Ability Hit?` (`/Game/Blueprints/AI/Base/BP_AICharacter_Base.Calculate Ability Hit` (`self.Character`) (`local.Ability Target`) (`self.Ability Difficulty`)))
  (`|SpawnActorFromClass` "/Game/Blueprints/Abilities/SpawnActors/BP_ShootingStar.BP_ShootingStar_C" (`self.GetTransform` _ability_target) "Undefined" "OverrideRootScale" null _ability_target (`self.Character`) (`self.Ability Difficulty`) (`/Game/Blueprints/AI/Base/BP_AICharacter_Base.Calculate Ability Damage` (`self.Character`) (`self.Damage Base`)) (`self.Is Ability Hit?`) null))

(fn `UserConstructionScript`
  (`parent.UserConstructionScript`))