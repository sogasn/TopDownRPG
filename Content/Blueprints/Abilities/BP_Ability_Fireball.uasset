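; Fireball ability Blueprint that launches a BP_FireBall projectile from the casting character toward the ability cursor location.
; It overrides the parent's projectile spawn, calling the parent first, then asking the Character to calculate hit success from target and difficulty.
; The projectile spawns at the Character's AbilitySpawner, rotated toward the cursor, and receives the hit result and Character-calculated damage at spawn.
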(event `self.ReceiveBeginPlay`
  (`parent.ReceiveBeginPlay`))

(fn `Spawn Ability Projectile`
  (params (`Ability Target` :type "/Game/Blueprints/AI/Base/BP_AICharacter_Base Object Reference"))
  (bind (_returnvalue_location _returnvalue_rotation _returnvalue_scale) (`KismetMathLibrary.BreakTransform` (`SceneComponent.K2_GetComponentToWorld` (`/Game/Blueprints/AI/Base/BP_AICharacter_Base.Ability Spawner` (`self.Character`)))))
  (`parent.Spawn Ability Projectile` `Ability Target`)
  ;[1 1 1] Calculate Attack Value
  (set `self.Is Ability Hit?` (`/Game/Blueprints/AI/Base/BP_AICharacter_Base.Calculate Ability Hit` (`self.Character`) (`local.Ability Target`) (`self.Ability Difficulty`)))
  ;[1 1 1] Spawn Ability Actor
  (`|SpawnActorFromClass` "/Game/Blueprints/Abilities/SpawnActors/BP_FireBall.BP_FireBall_C" (`KismetMathLibrary.MakeTransform` _returnvalue_location (`KismetMathLibrary.FindLookAtRotation` _returnvalue_location (`self.Ability Cursor Location`)) _returnvalue_scale) "AdjustIfPossibleButDontSpawnIfColliding" "OverrideRootScale" null (`/Game/Blueprints/AI/Base/BP_AICharacter_Base.Calculate Ability Damage` (`self.Character`) (`self.Damage Base`)) (`self.Is Ability Hit?`) null))

(fn `UserConstructionScript`
  (`parent.UserConstructionScript`))