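; Base Blueprint for a character class, providing a ten-level progression framework for child classes.
; AddLevel switches on Level to call one of ten per-level functions, all empty here as apparent override points.
; When IsEditorLevel is set, BeginPlay casts the parent actor to BP_AICharacter_Base, stores it as Pawn, and applies each level from 1 to LevelInEditor in order.
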(event `self.ReceiveBeginPlay`
  (if (`self.Is Editor Level?`)
    (bind _asbp_aicharacter_base (cast `/Game/Blueprints/AI/BP_AICharacter_Base` (`self.GetAttachParentActor`)))
    (set `self.Pawn` _asbp_aicharacter_base)
    (for _index (range 1 (+ (`self.Level In Editor`) 1))
      (set `self.Level` _index)
      (`self.Add Level`))))

(fn `Add Level`
  (switch `int` (`self.Level`)
    (:`1`
      (`self.Add Level 1`))
    (:`2`
      (`self.Add Level  2`))
    (:`3`
      (`self.Add Level  3`))
    (:`4`
      (`self.Add Level 4`))
    (:`5`
      (`self.Add Level 5`))
    (:`6`
      (`self.Add Level 6`))
    (:`7`
      (`self.Add Level 7`))
    (:`8`
      (`self.Add Level 8`))
    (:`9`
      (`self.Add Level 9`))
    (:`10`
      (`self.Add Level 10`))))

(fn `Add Level  2`)

(fn `Add Level  3`)

(fn `Add Level 1`)

(fn `Add Level 10`)

(fn `Add Level 4`)

(fn `Add Level 5`)

(fn `Add Level 6`)

(fn `Add Level 7`)

(fn `Add Level 8`)

(fn `Add Level 9`)

(fn `UserConstructionScript`)