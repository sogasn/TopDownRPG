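; BP_Class_Fighter is the Fighter character class Blueprint, a child class that overrides the level-up functions for levels 1 through 10.
; Each Add Level function calls its parent, then runs the shared Switch On Subclass macro, which branches on FighterSubclass into Knight or Duelist.
; Nothing follows either branch in any level, so it is a scaffold with no Fighter-specific or subclass-specific level logic yet.
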(fn `Add Level  2`
  (`parent.Add Level  2`)
  (`self.Switch On Subclass`))

(fn `Add Level  3`
  (`parent.Add Level  3`)
  (`self.Switch On Subclass`))

(fn `Add Level 1`
  (`parent.Add Level 1`)
  (`self.Switch On Subclass`))

(fn `Add Level 10`
  (`parent.Add Level 10`)
  (`self.Switch On Subclass`))

(fn `Add Level 4`
  (`parent.Add Level 4`)
  (`self.Switch On Subclass`))

(fn `Add Level 5`
  (`parent.Add Level 5`)
  (`self.Switch On Subclass`))

(fn `Add Level 6`
  (`parent.Add Level 6`)
  (`self.Switch On Subclass`))

(fn `Add Level 7`
  (`parent.Add Level 7`)
  (`self.Switch On Subclass`))

(fn `Add Level 8`
  (`parent.Add Level 8`)
  (`self.Switch On Subclass`))

(fn `Add Level 9`
  (`parent.Add Level 9`)
  (`self.Switch On Subclass`))

(fn `UserConstructionScript`
  (`parent.UserConstructionScript`))