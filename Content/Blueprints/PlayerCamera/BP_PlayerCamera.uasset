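; Player camera pawn for a party RPG, handling pan, zoom, rotation, HUD, pause, inventory and vendor UI.
; Left-click takes control of a character; right-click writes targets to its AI blackboard, repeating on a timer while held outside combat.
; An optional follow mode snaps the camera to that character through a looping tiny Delay.
; It also tracks turn-based fights with initiative sorting and round counting, though StartTurn is empty.
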(event `InputAction|Left Mouse Button` :paused true
  (params (Key :type "Key Structure"))
  (bind (_bblockinghit _binitialoverlap _time _distance _location _impactpoint _normal _impactnormal _physmat _hitactor) (`GameplayStatics.BreakHitResult` (`self.Get Hit Result Under Cursor`)))
  ;[1 1 1] Left Mouse Button
  (:`Pressed`
    (if (not (`self.Is Player In Dialogue?`))
      (if (`KismetSystemLibrary.DoesImplementInterface` _hitactor "/Game/Libraries/BPI_TakeControl.BPI_TakeControl_C")
        (bind _controlled_character (`self.Controlled Character`)
          (:`then`
            (bind _decal (`/Game/Blueprints/AI/BP_AICharacter_Base.Decal` _controlled_character))
            (`SceneComponent.SetVisibility` _decal false false)
            (`DecalComponent.SetDecalMaterial` _decal null))
          (:`else`
            _))
        (message `/Game/Libraries/BPI_TakeControl.Take Control` _hitactor)
        (bind _asbp_aicharacter_base (cast `/Game/Blueprints/AI/BP_AICharacter_Base` _hitactor))
        (set `self.Controlled Character` _asbp_aicharacter_base)))))

(event `InputAction|Display Object Names` :paused true
  (params (Key :type "Key Structure"))
  ;[1 1 1] Display Object Names
  (:`Pressed`
    (bind _outactors (`GameplayStatics.GetAllActorsWithTag` "Has Name Displayed"))
    (for _array_element _outactors
      (message `/Game/Libraries/BPI_Interact.Toggle Widget Name` _array_element true)))
  (:`Released`
    (bind _outactors_2 (`GameplayStatics.GetAllActorsWithTag` "Has Name Displayed"))
    (for _array_element_2 _outactors_2
      (message `/Game/Libraries/BPI_Interact.Toggle Widget Name` _array_element_2 false))))

(event `InputAction|Pause Game` :paused true
  (params (Key :type "Key Structure"))
  ;[1 1 1] Pause Game
  (:`Pressed`
    (if (not (`self.Is Player In Dialogue?`))
      (`/Game/Blueprints/Inventory/AC_Inventory.Inventory Panel` (`self.Party Inventory`)
        (:`then`)
        (:`else`
          (`GameplayStatics.SetGamePaused` (not (`GameplayStatics.IsGamePaused`))))))))

(event `InputAxis|Move Forward`
  (params (AxisValue :type "Float (single-precision)"))
  ;[1 1 1] Camera Movement
  (`PawnMovementComponent.AddInputVector` (`self.FloatingPawnMovement`) (* AxisValue (`KismetMathLibrary.GetForwardVector` (`self.K2_GetActorRotation`))) false))

(event `InputAxis|Move Right`
  (params (AxisValue :type "Float (single-precision)"))
  ;[1 1 1] Camera Movement
  (`PawnMovementComponent.AddInputVector` (`self.FloatingPawnMovement`) (* AxisValue (`KismetMathLibrary.GetRightVector` (`self.K2_GetActorRotation`))) false))

(event `InputAxis|Scroll Axis`
  (params (AxisValue :type "Float (single-precision)"))
  (bind _springarm (`self.SpringArm`))
  ;[1 1 1] Camera Movement
  (set `SpringArmComponent.TargetArmLength` (`KismetMathLibrary.FClamp` (+ AxisValue (`SpringArmComponent.TargetArmLength` _springarm)) (`self.Target Arm Min Length`) (`self.Target Arm Max Length`)) _springarm))

(event `InputAxis|Rotate Camera`
  (params (AxisValue :type "Float (single-precision)"))
  (bind (_returnvalue_roll _returnvalue_pitch _returnvalue_yaw) (`KismetMathLibrary.BreakRotator` (`self.K2_GetActorRotation`)))
  ;[1 1 1] Camera Movement
  (`self.K2_SetActorRotation` (`KismetMathLibrary.MakeRotator` _returnvalue_roll _returnvalue_pitch (+ AxisValue _returnvalue_yaw))))

(event `InputAction|Middle Mouse Button`
  (params (Key :type "Key Structure"))
  ;[1 1 1] Camera Movement
  (:`Pressed`
    (set `self.Middle Button Pressed` true))
  (:`Released`
    (set `self.Middle Button Pressed` false)))

(event `InputAxisKey|MouseX`
  (params (AxisValue :type "Float (single-precision)"))
  (bind (_returnvalue_roll _returnvalue_pitch _returnvalue_yaw) (`KismetMathLibrary.BreakRotator` (`self.K2_GetActorRotation`)))
  ;[1 1 1] Camera Movement
  (if (`self.Middle Button Pressed`)
    (`self.K2_SetActorRotation` (`KismetMathLibrary.MakeRotator` _returnvalue_roll _returnvalue_pitch (+ _returnvalue_yaw (* (`self.GetInputAxisKeyValue`) (`self.Mouse X Multiplier`)))))))

(event `InputAction|Follow Camera`
  (params (Key :type "Key Structure"))
  ;[1 1 1] Camera Movement
  (:`Pressed`
    (`self.Controlled Character`
      (:`then`
        (set `self.Is Camera Follows Character?` (not (`self.Is Camera Follows Character?`))))
      (:`else`))))

(event `self.ReceiveBeginPlay`
  ;[1 1 1] Initial Setup
  (`|ExecutionSequence`
    (:`then_0`
      (bind _returnvalue (`|CreateWidget` "/Game/HUD/UMG_GameHUD.UMG_GameHUD_C"))
      (bind _output_get (set `self.Player HUD` _returnvalue))
      (`UserWidget.AddToPlayerScreen` _output_get 0)
      (`WidgetBlueprintLibrary.SetInputMode_GameAndUIEx` (`GameplayStatics.GetPlayerController` 0) null "DoNotLock" false))
    (:`then_1`
      (`self.Toggle Camera Follows Controlled Character`))))

(event `InputAction|Inventory` :paused true
  (params (Key :type "Key Structure"))
  ;[1 1 1] Toggle Inventory
  (:`Pressed`
    (if (not (`self.Is Player In Dialogue?`))
      (`/Game/Blueprints/Inventory/AC_Inventory.Toggle Inventory` (`self.Party Inventory`) null)
      (`KismetSystemLibrary.K2_ClearTimer` null "Right Mouse Button"))))

(event `InputAction|Right Mouse Button` :paused true
  (params (Key :type "Key Structure"))
  ;[1 1 1] Right Mouse Button
  (:`Pressed`
    (`self.Check If Character Is In Fight`
      (:`Is In Fight And Controlled Character Is Player Controlled`
        _)
      (:`Is Not In Fight`
        _))
    (if (not (`self.Is Player In Dialogue?`))
      (`self.Right Mouse Button`)
      (if (not (`self.Is In Fight`))
        (`KismetSystemLibrary.K2_SetTimer` null "Right Mouse Button" 0.15 true))))
  (:`Released`
    (`KismetSystemLibrary.K2_ClearTimer` null "Right Mouse Button")))

(fn `End Fight`
  (set `self.Is In Fight` false)
  (`KismetArrayLibrary.Array_Clear` (`self.Characters In Battle`)))

(fn `End Turn`
  ;[1 1 1] If Character Is Last In Array...
  (if (== (`KismetArrayLibrary.Array_LastIndex` (`self.Characters In Battle`)) (`self.Current Character Moving Index`))
    ;[1 1 1] ...Start New Turn
    (`self.Start Round`)
    (`self.Start Turn` 0)
    (return)
    (else
      ;[1 1 1] ...Or Select Next Character In Array
      (bind _result (`/Engine/EditorBlueprintResources/StandardMacros.IncrementInt` (`self.Current Character Moving Index`))
        (:`  `
          (`self.Start Turn` _result)
          (return))))))

(fn `Filter Character By Initiative`
  (params (Characters :type "Array of /Game/Blueprints/AI/BP_AICharacter_Base Object Reference"))
  (returns (`Return Array` :type "Array of /Game/Blueprints/AI/BP_AICharacter_Base Object Reference"))
  (locals (`Array: Characters` :type "Array of /Game/Blueprints/AI/BP_AICharacter_Base Object Reference") (`Array: Initiative` :type "Array of Integer") (`New Array` :type "Array of /Game/Blueprints/AI/BP_AICharacter_Base Object Reference") (Index :type Integer))
  (bind _output_get (set `local.Array: Characters` Characters))
  ;[1 1 1] Create Array With Initiative Value
  (if (!= (`KismetArrayLibrary.Array_Length` _output_get) (`KismetArrayLibrary.Array_Length` (`local.Array: Initiative`))) :!label _label
    (`KismetArrayLibrary.Array_AddUnique` (`local.Array: Initiative`) (`/Game/Blueprints/Stats/AC_CharacterStats.Initiative` (`/Game/Blueprints/AI/BP_AICharacter_Base.Character Stats` (`|GetArrayItem` (`local.Array: Characters`) (`local.Index`)))))
    (`/Engine/EditorBlueprintResources/StandardMacros.IncrementInt` (`local.Index`)
      (:`  `
        (goto _label)))
    (else
      ;[1 1 1] Filter Iniriative Array
      (set `local.Index` 0)
      (bind _filtered_array (`self.Filter Int Array` (`local.Array: Initiative`) true))
      (bind _output_get_2 (set `local.Array: Initiative` _filtered_array))
      ;[1 1 1] Creaye New Character Array Based On Initiative
      (if (!= (`KismetArrayLibrary.Array_Length` _output_get_2) (`local.Index`)) :!label _label_2
        (for _array_element (`local.Array: Characters`)
          (if (== (`/Game/Blueprints/Stats/AC_CharacterStats.Initiative` (`/Game/Blueprints/AI/BP_AICharacter_Base.Character Stats` _array_element)) (`|GetArrayItem` (`local.Array: Initiative`) (`local.Index`)))
            (`KismetArrayLibrary.Array_AddUnique` (`local.New Array`) _array_element)
            (`/Engine/EditorBlueprintResources/StandardMacros.IncrementInt` (`local.Index`)
              (:`  `
                (goto _label_2)))))
        (else
          (return (`local.New Array`)))))))

(fn `Filter Int Array`
  (params (`Int Array` :type "Array of Integer") (`Sort Descending?` :type Boolean))
  (returns (`Filtered Array` :type "Array of Integer"))
  (locals (`Initial Array` :type "Array of Integer") (`New Array` :type "Array of Integer"))
  (bind _new_array (`local.New Array`))
  (bind _new_array_2 (`local.New Array`))
  (bind _initial_array (`local.Initial Array`))
  (bind _initial_array_2 (`local.Initial Array`))
  (bind (_indexofmaxvalue _maxvalue) (`KismetMathLibrary.MaxOfIntArray` _initial_array))
  (bind (_indexofminvalue _minvalue) (`KismetMathLibrary.MinOfIntArray` _initial_array_2))
  (set `local.Initial Array` `Int Array`)
  (if `Sort Descending?`
    (if (`KismetArrayLibrary.Array_IsNotEmpty` _initial_array_2) :!label _label
      (`KismetArrayLibrary.Array_Set` _new_array_2 (+ (`KismetArrayLibrary.Array_LastIndex` _new_array_2) 1) _minvalue true)
      (`KismetArrayLibrary.Array_Remove` _initial_array_2 _indexofminvalue)
      (goto _label)
      (else
        (return (`local.New Array`))))
    (else
      (if (`KismetArrayLibrary.Array_IsNotEmpty` _initial_array) :!label _label_2
        (`KismetArrayLibrary.Array_Set` _new_array (+ (`KismetArrayLibrary.Array_LastIndex` _new_array) 1) _maxvalue true)
        (`KismetArrayLibrary.Array_Remove` _initial_array _indexofmaxvalue)
        (goto _label_2)
        (else
          (return (`local.New Array`)))))))

(fn `Get Hit Result Under Cursor`
  (returns (HitResult :type "HitResult Structure") (ReturnValue :type Boolean))
  (bind (_hitresult _returnvalue) (`PlayerController.GetHitResultUnderCursorByChannel` (`GameplayStatics.GetPlayerController` 0) "TraceTypeQuery2" true))
  (return _hitresult _returnvalue))

(fn `Is Player In Dialogue?`
  (returns (`Return Value` :type Boolean))
  (return (`/Game/HUD/UMG_GameHUD.Is Dialogue?` (`self.Player HUD`))))

(fn `Right Mouse Button`
  (bind (_bblockinghit _binitialoverlap _time _distance _location _impactpoint _normal _impactnormal _physmat _hitactor) (`GameplayStatics.BreakHitResult` (`self.Get Hit Result Under Cursor`)))
  (bind _controlled_character (`self.Controlled Character`)
    (:`then`
      (if (`|EnumEquality` (`/Game/Blueprints/AI/BP_AICharacter_Base.Attitude Towards Player` _controlled_character) "NewEnumerator3")
        (if (not (`KismetSystemLibrary.DoesImplementInterface` _hitactor "/Game/Libraries/BPI_Interact.BPI_Interact_C"))
          ;[1 0.008681 0] When Player Use Right Mouse Button On Something That Doesn't Implement Interact Interface
          (`BlackboardComponent.SetValueAsVector` (`AIBlueprintHelperLibrary.GetBlackboard` (`AIBlueprintHelperLibrary.GetAIController` (`self.Controlled Character`))) "Target Location" _location)
          ;[1 1 1 1 20] Draw Cursor
          (`NiagaraFunctionLibrary.SpawnSystemAtLocation` (`self.FXCursor`) _location :!label _label)
          (elif (not (== (`self.Controlled Character`) _hitactor))
            (`BlackboardComponent.SetValueAsObject` (`AIBlueprintHelperLibrary.GetBlackboard` (`AIBlueprintHelperLibrary.GetAIController` (`self.Controlled Character`))) "Interacted Actor" _hitactor)
            (`BlackboardComponent.SetValueAsVector` (`AIBlueprintHelperLibrary.GetBlackboard` (`AIBlueprintHelperLibrary.GetAIController` (`self.Controlled Character`))) "Target Location" _location)
            (goto _label)))))
    (:`else`)))

(fn `Start Fight`
  (params (`Characters To Fight` :type "Array of /Game/Blueprints/AI/BP_AICharacter_Base Object Reference"))
  ;[1 1 1] Prepare For Fight
  (set `self.Is In Fight` true)
  (bind _return_array (`self.Filter Character By Initiative` `Characters To Fight`))
  (bind _output_get (set `self.Characters In Battle` _return_array))
  (for _array_element _output_get
    (`/Game/Blueprints/AI/BP_AICharacter_Base.Set Combat Pose` _array_element true)
    (bind _mesh (`Character.Mesh` _array_element))
    (`PrimitiveComponent.SetRenderCustomDepth` _mesh true)
    (`PrimitiveComponent.SetCustomDepthStencilValue` _mesh 1)
    (set `self.Current Turn` 1)
    (set `self.Current Character Moving Index` 0)))

(fn `Start Round`
  (set `self.Current Character Moving Index` 0)
  (`/Engine/EditorBlueprintResources/StandardMacros.IncrementInt` (`self.Current Turn`)
    (:`  `
      (return))))

(fn `Start Turn`
  (params (`Character Index` :type Integer)))

(fn `Toggle Vendor`
  (params (`Vendor Inventory` :type "/Game/Blueprints/Inventory/AC_Inventory Object Reference") (`Display Shop` :type "/Game/Blueprints/AI/Tasks/BTT_DisplayShop Object Reference"))
  (bind _vendor (`self.Vendor`)
    (:`then`
      (`Widget.RemoveFromParent` _vendor)
      (set `self.Vendor` null))
    (:`else`
      (bind _returnvalue (`|CreateWidget` "/Game/HUD/Vendor/UMG_Vendor.UMG_Vendor_C" null (`self.Party Inventory`) `Vendor Inventory` `Display Shop`))
      (bind _output_get (set `self.Vendor` _returnvalue))
      (`UserWidget.AddToPlayerScreen` _output_get 0)))
  (return))

(fn `UserConstructionScript`)