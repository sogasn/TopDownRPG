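; Character stats component for an RPG, holding seven attributes, armor class, magic resistance, health, experience and skills.
; Attribute changes recompute diminishing-returns percentage modifiers, with Agility and Wisdom feeding armor class (including a Monk formula) and Wisdom feeding magic resistance.
; Skill checks add a Luck-adjusted random roll to the skill and its governing modifier, except Persuasion, which gets no modifier.
; Exceeding the experience threshold only grants a level-up point.
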(fn `Add Agility`
  (params (`Agility To Add` :type Integer))
  (set `self.Agility` (+ `Agility To Add` (`self.Agility`)))
  (`self.Set Agility Modifier`)
  (return))

(fn `Add Armor`
  (params (`Armor To Add` :type Integer))
  (set `self.Armor Class` (+ `Armor To Add` (`self.Armor Class`)))
  (return))

(fn `Add Armor from Clothes`
  (params (`Armor To Add` :type Integer) (`Agility Penalty` :type Integer))
  ;[1 1 1] Add Armor Class From Item And Agility Penalty (If Has Penalty)
  (set `self.Armor: Clothes` (+ `Armor To Add` (`self.Armor: Clothes`)))
  (set `self.Agility Penalty For Armor` (- (`self.Agility Penalty For Armor`) (`local.Agility Penalty`)))
  (`self.Set Armor`)
  (return))

(fn `Add Charisma`
  (params (`Charisma To Add` :type Integer))
  (set `self.Charisma` (+ `Charisma To Add` (`self.Charisma`)))
  (`self.Set Charisma Modifier`)
  (return))

(fn `Add Constitution`
  (params (`Constitution To Add` :type Integer))
  (set `self.Constitution` (+ `Constitution To Add` (`self.Constitution`)))
  (`self.Set Constitution Modifier`)
  (return))

(fn `Add Exp`
  (params (`Experience To Add` :type Integer))
  (bind _output_get (set `self.Experience` (+ `Experience To Add` (`self.Experience`))))
  (if (> _output_get (`self.Experience To Next Level`))
    (`self.LevelUP`)
    (return)
    (else
      (return))))

(fn `Add Health`
  (params (`Health To Add` :type Integer))
  (set `self.HP` (`KismetMathLibrary.Clamp` (+ `Health To Add` (`self.HP`)) 0 (`self.HP Max`)))
  (return))

(fn `Add Intelligence`
  (params (`Intelligence To Add` :type Integer))
  (set `self.Intelligence` (+ `Intelligence To Add` (`self.Intelligence`)))
  (`self.Set Intelligence Modifier`)
  (return))

(fn `Add Luck`
  (params (`Luck To Add` :type Integer))
  (set `self.Luck` (+ `Luck To Add` (`self.Luck`)))
  (`self.Set Luck Modifier`)
  (return))

(fn `Add Magic Resistance`
  (params (`Resistance To Add` :type Integer))
  (set `self.Magic Resistance` (+ `Resistance To Add` (`self.Magic Resistance`)))
  (return))

(fn `Add Magic Resistance from Clothes`
  (params (`Resistance To Add` :type Integer))
  (set `self.Magic Resistance: Clothes` (+ `Resistance To Add` (`self.Magic Resistance: Clothes`)))
  (`self.Set Magic Resistance`)
  (return))

(fn `Add Strength`
  (params (`Strength To Add` :type Integer))
  (set `self.Strength` (+ `Strength To Add` (`self.Strength`)))
  (`self.Set Strength Modifier`)
  (return))

(fn `Add Wisdom`
  (params (`Wisdom To Add` :type Integer))
  (set `self.Wisdom` (+ `Wisdom To Add` (`self.Wisdom`)))
  (`self.Set Wisdom Modifier`)
  (return))

(fn `Get Characteristic Modifier On Enum`
  (params (Characteristic :type "/Game/Blueprints/Stats/E_Characteristics Enum" :default "NewEnumerator0"))
  (returns (`Modifier Value` :type Integer))
  (return (select `/Game/Blueprints/Stats/E_Characteristics` Characteristic :`NewEnumerator0` (`self.Strength Modifier`) :`NewEnumerator1` (`self.Agility Modifier`) :`NewEnumerator2` (`self.Constitution Modifier`) :`NewEnumerator3` (`self.Intelligence Modifier`) :`NewEnumerator4` (`self.Wisdom Modifier`) :`NewEnumerator5` (`self.Charisma Modifier`) :`NewEnumerator6` (`self.Luck Modifier`))))

(fn `Get Skill Value`
  (params (NewParam :type "/Game/Blueprints/Stats/E_Skills Enum" :default "NewEnumerator0"))
  (returns (`Skill Value` :type Integer))
  (bind _rng_value (`self.Throw RNG DICE`))
  (return (+ _rng_value (select `/Game/Blueprints/Stats/E_Skills` NewParam :`NewEnumerator0` (+ (`self.Athletics`) (`self.Strength Modifier`)) :`NewEnumerator1` (+ (`self.Stealth`) (`self.Agility Modifier`)) :`NewEnumerator2` (+ (`self.Trickery`) (`self.Agility Modifier`)) :`NewEnumerator3` (+ (`self.Knowlege`) (`self.Intelligence Modifier`)) :`NewEnumerator4` (+ (`self.Perception`) (`self.Wisdom Modifier`)) :`NewEnumerator5` (+ (`self.First Aid`) (`self.Wisdom Modifier`)) :`NewEnumerator6` (+ (`self.Persuasion`) 0)))))

(fn `Is Character Dead?`
  (returns (`Is Dead` :type Boolean))
  (return (<= (`self.HP`) 0)))

(fn `LevelUP`
  (`/Engine/EditorBlueprintResources/StandardMacros.IncrementInt` (`self.LVLUP Points`)
    (:`  `
      (return))))

(fn `Remove Agility`
  (params (`Agility To Remove` :type Integer))
  (set `self.Agility` (- (`self.Agility`) `Agility To Remove`))
  (`self.Set Agility Modifier`)
  (return))

(fn `Remove Armor`
  (params (`Armor To Remove` :type Integer))
  (set `self.Armor Class` (- (`self.Armor Class`) `Armor To Remove`))
  (return))

(fn `Remove Armor Clothes`
  (params (`Armor To Remove` :type Integer) (`Agility Penalty` :type Integer))
  ;[1 1 1] Remove Armor From Item (and Restore Agility Modifier)
  (set `self.Armor: Clothes` (- (`self.Armor: Clothes`) `Armor To Remove`))
  (set `self.Agility Penalty For Armor` (+ (`self.Agility Penalty For Armor`) (`local.Agility Penalty`)))
  (`self.Set Armor`)
  (return))

(fn `Remove Charisma`
  (params (`Charisma To Remove` :type Integer))
  (set `self.Charisma` (- (`self.Charisma`) `Charisma To Remove`))
  (`self.Set Charisma Modifier`)
  (return))

(fn `Remove Constitution`
  (params (`Constitution To Remove` :type Integer))
  (set `self.Constitution` (- (`self.Constitution`) `Constitution To Remove`))
  (`self.Set Constitution Modifier`)
  (return))

(fn `Remove Health`
  (params (`Health To Remove` :type Integer))
  (returns (`Is HP Below Zero?` :type Boolean))
  (bind _output_get (set `self.HP` (- (`self.HP`) `Health To Remove`)))
  (return (<= _output_get 0)))

(fn `Remove Intelligence`
  (params (`Intelligence To Remove` :type Integer))
  (set `self.Intelligence` (- (`self.Intelligence`) `Intelligence To Remove`))
  (`self.Set Intelligence Modifier`)
  (return))

(fn `Remove Luck`
  (params (`Luck To Remove` :type Integer))
  (set `self.Luck` (- (`self.Luck`) `Luck To Remove`))
  (`self.Set Luck Modifier`)
  (return))

(fn `Remove Magic Resistance`
  (params (`Resistance To Remove` :type Integer))
  (set `self.Magic Resistance` (- (`self.Magic Resistance`) `Resistance To Remove`))
  (return))

(fn `Remove Magic Resistance Clothes`
  (params (`Resistance To Remove` :type Integer))
  (set `self.Magic Resistance: Clothes` (- (`self.Magic Resistance: Clothes`) `Resistance To Remove`))
  (`self.Set Magic Resistance`)
  (return))

(fn `Remove Strength`
  (params (`Strength To Remove` :type Integer))
  (set `self.Strength` (- (`self.Strength`) `Strength To Remove`))
  (`self.Set Strength Modifier`)
  (return))

(fn `Remove Wisdom`
  (params (`Wisdom To Add` :type Integer))
  (set `self.Wisdom` (- (`self.Wisdom`) `Wisdom To Add`))
  (`self.Set Wisdom Modifier`)
  (return))

(fn `Set Agility Modifier`
  (bind _returnvalue (`KismetMathLibrary.Conv_IntToDouble` (`self.Agility`)))
  (set `self.Agility Modifier` (`KismetMathLibrary.FFloor` (* (/ _returnvalue (+ _returnvalue (`self.Base Characristic Divider`))) 100.0)))
  (if (`self.Is Monk?`)
    (`self.Set Armor For Monk`)
    (else
      (`self.Set Armor`)))
  (return))

(fn `Set Armor`
  (if (`self.Is Monk?`)
    (if (or (`self.Is Vearing Armor`) (`self.Is Vearing Shield`))
      (set `self.Armor Class` (+ (`self.Armor: Clothes`) (- (`self.Agility Modifier`) (`self.Agility Penalty For Armor`))) :!label _label)
      (return)
      (else
        (`self.Set Armor For Monk`)))
    (else
      (goto _label))))

(fn `Set Armor For Monk`
  (set `self.Armor Class` (+ (`self.Wisdom Modifier`) (`self.Agility Modifier`) 5))
  (return))

(fn `Set Charisma Modifier`
  (bind _returnvalue (`KismetMathLibrary.Conv_IntToDouble` (`self.Charisma`)))
  (set `self.Charisma Modifier` (`KismetMathLibrary.FFloor` (* (/ _returnvalue (+ _returnvalue (`self.Base Characristic Divider`))) 100.0)))
  (return))

(fn `Set Constitution Modifier`
  (bind _returnvalue (`KismetMathLibrary.Conv_IntToDouble` (`self.Constitution`)))
  (set `self.Constitution Modifier` (`KismetMathLibrary.FFloor` (* (/ _returnvalue (+ _returnvalue (`self.Base Characristic Divider`))) 100.0)))
  (return))

(fn `Set Intelligence Modifier`
  (bind _returnvalue (`KismetMathLibrary.Conv_IntToDouble` (`self.Intelligence`)))
  (set `self.Intelligence Modifier` (`KismetMathLibrary.FFloor` (* (/ _returnvalue (+ _returnvalue (`self.Base Characristic Divider`))) 100.0))))

(fn `Set Luck Modifier`
  (bind _returnvalue (`KismetMathLibrary.Conv_IntToDouble` (`self.Luck`)))
  (set `self.Luck Modifier` (`KismetMathLibrary.FFloor` (* (/ (- _returnvalue 20.0) (+ _returnvalue (`self.Luck Divider`))) 100.0)))
  (return))

(fn `Set Magic Resistance`
  (set `self.Magic Resistance` (+ (`self.Magic Resistance: Clothes`) (`self.Wisdom Modifier`)))
  (return))

(fn `Set Strength Modifier`
  (bind _returnvalue (`KismetMathLibrary.Conv_IntToDouble` (`self.Strength`)))
  (set `self.Strength Modifier` (`KismetMathLibrary.FFloor` (* (/ _returnvalue (+ _returnvalue (`self.Base Characristic Divider`))) 100.0)))
  (return))

(fn `Set Wisdom Modifier`
  (bind _returnvalue (`KismetMathLibrary.Conv_IntToDouble` (`self.Wisdom`)))
  (set `self.Wisdom Modifier` (`KismetMathLibrary.FFloor` (* (/ _returnvalue (+ _returnvalue (`self.Base Characristic Divider`))) 100.0)))
  (`self.Set Magic Resistance`)
  (if (`self.Is Monk?`)
    (`self.Set Armor For Monk`))
  (return))

(fn `Throw RNG DICE`
  (returns (`RNG Value` :type Integer))
  (bind _output_get (set `self.RNG` (+ (`KismetMathLibrary.RandomIntegerInRange` (`self.Min RNG Value`) (`self.Max RNG Value`)) (`self.Luck Modifier`))))
  (return _output_get))