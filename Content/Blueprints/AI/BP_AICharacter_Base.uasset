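; Base AI character for an RPG, handling dice-based combat, equipment, player control and cursor feedback.
; Attack chains up to three strikes between montages, comparing attack and defence rolls to trigger melee damage or deflection.
; A looping timer derives battle pose from equipped weapons, which, with caster class, selects attack, block, hit and death montages.
; Hovering shows an attitude-coloured decal and camera-scaled name/health widget; interacting with non-hostiles runs a dialogue behavior tree.
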(event `self.ReceiveBeginPlay`
  (bind _ai_inventory (`self.AI Inventory`))
  ;[1 1 1] Begin Play
  (`AIController.RunBehaviorTree` (`AIBlueprintHelperLibrary.GetAIController` self) (`self.BT Under Player Control`))
  (bind _as_player (`/Game/Libraries/BlueprintFunctionLibrary.Cast To Player` 0))
  (set `self.Player Cast` _as_player)
  (bind _asumg_object_name (cast `/Game/HUD/UMG_ObjectName` (`WidgetComponent.GetWidget` (`self.Widget`))))
  (set `self.Object Widget` _asumg_object_name)
  (set `/Game/Blueprints/Inventory/AC_Inventory.Inventory` (`self.Inventory`) _ai_inventory)
  (set `/Game/Blueprints/Inventory/AC_Inventory.Money` (`self.Money`) _ai_inventory)
  (set `/Game/Blueprints/Inventory/AC_Inventory.Inventory Name` (`self.Name`) _ai_inventory)
  (`KismetSystemLibrary.K2_SetTimer` null "Pose Tracker" 0.3 true))

(event `Event Attack`
  (params (Attacked :type "/Game/Blueprints/AI/BP_AICharacter_Base Object Reference"))
  ;[1 1 1] Event Attack
  (bind _finished_attack (`self.Attack` Attacked :!label _label))
  (if (not _finished_attack)
    (if (`self.Is NOT Active Montage`) :!label _label_2
      (`KismetSystemLibrary.Delay` 0.2)
      (goto _label)
      (else
        (`KismetSystemLibrary.Delay` 0.2)
        (goto _label_2)))))

(event `Event Deflect`
  ;[1 1 1] Event Deflect
  (`KismetSystemLibrary.Delay` 0.5)
  (`self.Deflect`))

(event `/Game/Libraries/BPI_TakeControl.Take Control`
  ;[1 1 1] Event Take Control
  (`self.Set Decal Material LMB`))

(event `/Game/Libraries/BPI_Interact.Interact`
  (params (Interacter :type "Actor Object Reference"))
  ;[1 1 1] Interaction
  (if (`|EnumInequality` (`self.Attitude Towards Player`) "NewEnumerator1")
    (`AIController.RunBehaviorTree` (`AIBlueprintHelperLibrary.GetAIController` self) (`self.Dialogue BT`))))

(event `self.ReceiveAnyDamage`
  (params (Damage :type "Float (single-precision)") (DamageType :type "DamageType Object Reference") (InstigatedBy :type "Controller Object Reference") (DamageCauser :type "Actor Object Reference"))
  ;[1 1 1] Take Damage
  (`KismetSystemLibrary.PrintString` (`KismetStringLibrary.Conv_DoubleToString` Damage))
  (`/Game/Blueprints/Stats/AC_CharacterStats.Remove Health` (`self.Character Stats`) (`KismetMathLibrary.FTrunc` Damage)))

(event `Event Take Damage`
  (params (Damage :type Integer))
  ;[1 1 1] Take Damage
  (`KismetSystemLibrary.Delay` 0.5)
  (`GameplayStatics.ApplyDamage` self (`KismetMathLibrary.Conv_IntToDouble` Damage))
  (`self.Take Damage`)
  (if (`/Game/Blueprints/Stats/AC_CharacterStats.Is Character Dead?` (`self.Character Stats`))
    (`KismetSystemLibrary.Delay` (- (`self.Montage Length`) 0.3))
    (set `SkeletalMeshComponent.bPauseAnims` true (`self.Mesh`))))

(event `self.ReceiveActorBeginCursorOver`
  ;[1 1 1] Visual
  (if (!= (`/Game/Blueprints/PlayerCamera/BP_PlayerCamera.Controlled Character` (`self.Player Cast`)) self)
    (`self.Set Decal Hovered`))
  (`self.Set Object Widget Visible`)
  (`KismetSystemLibrary.K2_SetTimer` null "Set Object Widget Visible" 0.01 true))

(event `self.ReceiveActorEndCursorOver`
  ;[1 1 1] Visual
  (bind _as_player (`/Game/Libraries/BlueprintFunctionLibrary.Cast To Player` 0))
  (if (!= (`/Game/Blueprints/PlayerCamera/BP_PlayerCamera.Controlled Character` _as_player) self)
    (`SceneComponent.SetVisibility` (`self.Decal`) false false)
    (`DecalComponent.SetDecalMaterial` (`self.Decal`) null)
    (if (not (stale `/Game/Libraries/BPI_Interact.Toggle Widget Name` `Is Displaying?`))
      (`self.Hide Object Widget` :!label _label_3))
    (elif (not (stale `/Game/Libraries/BPI_Interact.Toggle Widget Name` `Is Displaying?`))
      (goto _label_3))))

(event `/Game/Libraries/BPI_Interact.Toggle Widget Name`
  (params (`Is Displaying?` :type Boolean))
  ;[1 1 1] Visual
  (if `Is Displaying?`
    (`self.Set Object Widget Visible`)
    (`KismetSystemLibrary.K2_SetTimer` null "Set Object Widget Visible" 0.01 true)
    (else
      (`self.Hide Object Widget`))))

(fn `Add To Equipment`
  (params (`Item To Add` :type "/Game/Blueprints/Pickables/BP_PickableItem_Base Object Reference"))
  ;[1 1 1] Add Item To Equipment
  (`KismetArrayLibrary.Array_AddUnique` (`self.Equipment`) `Item To Add`)
  ;[1 1 1] Check if item is shield, if true, set bool value in character stats
  (if (`|EnumEquality` (`.ItemType_18_4C884E6F4321BC5E70DF60ADCF90B142` (break `/Game/Blueprints/Inventory/ST_Item` (`/Game/Blueprints/Pickables/BP_PickableItem_Base.Item` (`local.Item To Add`)))) "NewEnumerator3")
    (set `/Game/Blueprints/Stats/AC_CharacterStats.Is Vearing Shield` true (`self.Character Stats`))
    (return)
    (else
      ;[1 1 1] If item is armor (cast is valid, has agility penalty), set bool value in character stats
      (bind _asbp_armor_base (cast `/Game/Blueprints/Pickables/Armor/BP_Armor_Base` (`local.Item To Add`))
        (:`then`
          (if (> (`/Game/Blueprints/Pickables/Armor/BP_Armor_Base.Penalty To Agility` _asbp_armor_base) 0)
            (set `/Game/Blueprints/Stats/AC_CharacterStats.Is Vearing Armor` true (`self.Character Stats`))
            (return)
            (else
              (return))))
        (:`CastFailed`
          (return))))))

(fn `Attack`
  (params (Attacked :type "/Game/Blueprints/AI/BP_AICharacter_Base Object Reference"))
  (returns (`Finished Attack` :type Boolean))
  (locals (`Attack Value` :type Integer) (`Defend Value` :type Integer) (Defender :type "/Game/Blueprints/AI/BP_AICharacter_Base Object Reference"))
  (bind _character_stats (`self.Character Stats`))
  (bind _character_stats_2 (`/Game/Blueprints/AI/BP_AICharacter_Base.Character Stats` (`local.Defender`)))
  (`self.Set Combat Pose` true)
  (`self.Set Combat Pose` Attacked true)
  (bind _output_get (set `local.Defender` Attacked))
  (if (not (`/Game/Blueprints/Stats/AC_CharacterStats.Is Character Dead?` (`/Game/Blueprints/AI/BP_AICharacter_Base.Character Stats` _output_get)))
    ;[1 1 1] Check Character Attack
    (if (`|EnumInequality` (`self.Current Attack`) "NewEnumerator3")
      (if (> (select `/Game/Blueprints/AI/E_Attack` (`self.Current Attack`) :`NewEnumerator0` (`self.First Attack Modifier`) :`NewEnumerator1` (`self.Second Attack Modifier`) :`NewEnumerator2` (`self.Third Attack Modifier`)) 0)
        ;[1 1 1] Calculate Attack
        (bind _rng_value (`/Game/Blueprints/Stats/AC_CharacterStats.Throw RNG DICE` _character_stats))
        (bind _output_get_2 (set `local.Attack Value` (+ _rng_value (`/Game/Blueprints/Stats/AC_CharacterStats.Get Characteristic Modifier On Enum` _character_stats (`self.Attack Characteristic`)) (select `/Game/Blueprints/AI/E_Attack` (`self.Current Attack`) :`NewEnumerator0` (`self.First Attack Modifier`) :`NewEnumerator1` (`self.Second Attack Modifier`) :`NewEnumerator2` (`self.Third Attack Modifier`)))))
        (`KismetSystemLibrary.PrintString` (`KismetStringLibrary.Conv_IntToString` _output_get_2))
        ;[1 1 1] Calculate Defence
        (bind _rng_value_2 (`/Game/Blueprints/Stats/AC_CharacterStats.Throw RNG DICE` _character_stats_2))
        (bind _output_get_3 (set `local.Defend Value` (+ _rng_value_2 (`/Game/Blueprints/Stats/AC_CharacterStats.Armor Class` _character_stats_2))))
        (`KismetSystemLibrary.PrintString` (`KismetStringLibrary.Conv_IntToString` _output_get_3))
        (`self.Attack Animation`)
        (if (not (`self.Is Ranged Weapon Equipped?`))
          ;[1 1 1] Compare Attack And Defecence Values
          (`/Engine/EditorBlueprintResources/StandardMacros.CompareInt` (`local.Attack Value`) (`local.Defend Value`)
            (:`>`
              (bind _attack_damage (`self.Claculate Attack From Weapon`))
              (`self.Event Take Damage` (`local.Defender`) _attack_damage))
            (:`==`
              (`self.Event Deflect` (`local.Defender`) :!label _label))
            (:`<`
              (goto _label)))
          (set `self.Current Attack` (select `/Game/Blueprints/AI/E_Attack` (`self.Current Attack`) :`NewEnumerator0` "NewEnumerator1" :`NewEnumerator1` "NewEnumerator2" :`NewEnumerator2` "NewEnumerator3" :`NewEnumerator3` "NewEnumerator3" :!type "/Game/Blueprints/AI/E_Attack Enum"))
          (return false))
        (else
          ;[1 1 1] If Attack Modifier Equals 0, Or All Attack Are Made, Character Cannot Attack This Turn
          (`KismetSystemLibrary.PrintString` "Cannot Attack" :!label _label_2)
          (return true)))
      (else
        (goto _label_2)))
    (else
      (return true))))

(fn `Attack Animation`
  ;[1 1 1] Check If Character Is NOT Caster
  (if (`self.Is NOT Caster?`)
    (`self.PlayAnimMontage` (`self.Get Attack Montage On Pose` (`self.Current Pose`)))
    (else
      ;[1 1 1] If Caster Play Attack Animation Based On Weapon
      (`self.PlayAnimMontage` (`self.Get Attack Montage On Pose` (`self.Battle Pose For Caster`)))))
  (return))

(fn `Claculate Attack From Weapon`
  (returns (`Attack Damage` :type Integer))
  (locals (Weapon :type "/Game/Blueprints/Pickables/BP_PickableItem_Base Object Reference") (`Characteristic Modifier` :type Integer :default 0))
  ;[1 1 1] If Character Has Weapon Equipped
  (for _array_element (`self.Equipment`)
    (if (`|EnumEquality` (`.ItemType_18_4C884E6F4321BC5E70DF60ADCF90B142` (break `/Game/Blueprints/Inventory/ST_Item` (`/Game/Blueprints/Pickables/BP_PickableItem_Base.Item` _array_element))) "NewEnumerator1")
      (set `local.Weapon` _array_element)
      (break)))
  (bind _weapon (`local.Weapon`)
    (:`then`
      (bind _asbp_weapon_base (cast `/Game/Blueprints/Pickables/Weapons/BP_Weapon_Base` _weapon))
      ;[1 1 1] Set Attack Value Based On Weapon Damage And Attck Characteristic Modifier
      (set `local.Characteristic Modifier` (`/Game/Blueprints/Stats/AC_CharacterStats.Get Characteristic Modifier On Enum` (`self.Character Stats`) (`/Game/Blueprints/Pickables/Weapons/BP_Weapon_Base.Weapon Damage Scale Characteristic` _asbp_weapon_base)))
      (`|ExecutionSequence`
        (:`then_0`
          (set `self.Attack Damage Max` (+ (`/Game/Blueprints/Pickables/Weapons/BP_Weapon_Base.Weapon Damage Max` _asbp_weapon_base) (`local.Characteristic Modifier`))))
        (:`then_1`
          (set `self.Attack Damage Min` (+ (`/Game/Blueprints/Pickables/Weapons/BP_Weapon_Base.Weapon Damage Min` _asbp_weapon_base) (`local.Characteristic Modifier`))))
        (:`then_2`
          ;[1 1 1] Add RNG Value To Attack
          (return (`self.Get Attack Value` (`self.Attack Damage Min`) (`self.Attack Damage Max`))))))
    (:`else`
      ;[1 1 1] Set Attack Value For Fists
      (return (`self.Get Attack Value` (`self.Attack Damage From Fists Min`) (`self.Attack Damage From Fists Max`))))))

(fn `Damage Animation`
  (if (`self.Is NOT Caster?`)
    (bind _returnvalue (`self.PlayAnimMontage` (`self.Get Damage Animation On Pose` (<= (`/Game/Blueprints/Stats/AC_CharacterStats.HP` (`self.Character Stats`)) 0) (`self.Battle Pose`))))
    (set `self.Montage Length` _returnvalue)
    (return)
    (else
      (bind _returnvalue_2 (`self.PlayAnimMontage` (`self.Get Damage Animation On Pose` (<= (`/Game/Blueprints/Stats/AC_CharacterStats.HP` (`self.Character Stats`)) 0) (`self.Battle Pose For Caster`))))
      (set `self.Montage Length` _returnvalue_2)
      (return))))

(fn `Deflect`
  (`self.Deflect Animation`))

(fn `Deflect Animation`
  (if (`self.Is NOT Caster?`)
    (`self.PlayAnimMontage` (`self.Get Deflect Animation On Pose` (`self.Battle Pose`)))
    (else
      (`self.PlayAnimMontage` (`self.Get Deflect Animation On Pose` (`self.Battle Pose For Caster`)))))
  (return))

(fn `Get Attack Montage On Pose`
  (params (Pose :type "/Game/Animations/E_Pose Enum" :default "NewEnumerator0"))
  (returns (ReturnValue :type "AnimMontage Object Reference"))
  (return (select `/Game/Animations/E_Pose` Pose :`NewEnumerator1` "/Game/Animations/Archer/AM_Archer_Shoot.AM_Archer_Shoot" :`NewEnumerator2` (select `int` (`KismetMathLibrary.RandomIntegerInRange` 0 2) :`0` "/Game/Animations/Fist/AM_Fist_Kicking.AM_Fist_Kicking" :`1` "/Game/Animations/Fist/AM_Fist_Punching_01.AM_Fist_Punching_01" :`2` "/Game/Animations/Fist/AM_Fist_Punching_02.AM_Fist_Punching_02" :!type "AnimMontage Object Reference") :`NewEnumerator3` (select `int` (`KismetMathLibrary.RandomIntegerInRange` 0 1) :`0` "/Game/Animations/GreatSword/AM_GreatSword_Slash_01.AM_GreatSword_Slash_01" :`1` "/Game/Animations/GreatSword/AM_GreatSword_Slash_02.AM_GreatSword_Slash_02" :!type "AnimMontage Object Reference") :`NewEnumerator4` "/Game/Animations/Fist/AM_Fist_Punching_01.AM_Fist_Punching_01" :`NewEnumerator5` (select `int` (`KismetMathLibrary.RandomIntegerInRange` 0 1) :`0` "/Game/Animations/OneHanded/AM_SwordAndShield_Slash.AM_SwordAndShield_Slash" :`1` "/Game/Animations/OneHanded/AM_SwordAndShield_Slash_02.AM_SwordAndShield_Slash_02" :!type "AnimMontage Object Reference") :`NewEnumerator6` (select `int` (`KismetMathLibrary.RandomIntegerInRange` 0 1) :`0` "/Game/Animations/Two-handedAxe/AM_TwoHAxe_Slash_01.AM_TwoHAxe_Slash_01" :`1` "/Game/Animations/Two-handedAxe/AM_TwoHAxe_Slash_02.AM_TwoHAxe_Slash_02" :!type "AnimMontage Object Reference"))))

(fn `Get Attack Value`
  (params (`Min Attack` :type Integer) (`Max Attack` :type Integer))
  (returns (`Attack Value` :type Integer))
  (locals (`RNG Value` :type Integer :default 0))
  ;[1 1 1] Add RNG Value To Random Number Between MAX and MIN Attack Values
  (bind _rng_value (`/Game/Blueprints/Stats/AC_CharacterStats.Throw RNG DICE` (`self.Character Stats`)))
  (set `local.RNG Value` _rng_value)
  (return (`KismetMathLibrary.Clamp` (+ (`KismetMathLibrary.RandomIntegerInRange` (`local.Min Attack`) (`local.Max Attack`)) (/ (`local.RNG Value`) 5)) (`local.Min Attack`) (`local.Max Attack`))))

(fn `Get Damage Animation On Pose`
  (params (`Is Death?` :type Boolean) (Pose :type "/Game/Animations/E_Pose Enum" :default "NewEnumerator0"))
  (returns (`Return Value` :type "AnimMontage Object Reference"))
  (if (not `Is Death?`)
    (return (select `/Game/Animations/E_Pose` (`local.Pose`) :`NewEnumerator1` "/Game/Animations/Archer/AM_Archer_Impact.AM_Archer_Impact" :`NewEnumerator2` "/Game/Animations/Fist/AM_Fist_Impact.AM_Fist_Impact" :`NewEnumerator3` "/Game/Animations/GreatSword/AM_GreatSword_Impact.AM_GreatSword_Impact" :`NewEnumerator4` "/Game/Animations/Magic/AM_Magic_Impact.AM_Magic_Impact" :`NewEnumerator5` "/Game/Animations/OneHanded/AM_SwordAndShield_Impact.AM_SwordAndShield_Impact" :`NewEnumerator6` "/Game/Animations/Two-handedAxe/AM_TwoHAxe_Impact.AM_TwoHAxe_Impact" :!type "AnimMontage Object Reference"))
    (else
      (`ActorComponent.Deactivate` (`self.CharacterMovement`))
      (return (select `/Game/Animations/E_Pose` (`local.Pose`) :`NewEnumerator0` "/Game/Animations/Archer/AM_Archer_Death.AM_Archer_Death" :`NewEnumerator1` "/Game/Animations/Archer/AM_Archer_Death.AM_Archer_Death" :`NewEnumerator2` "/Game/Animations/Archer/AM_Archer_Death.AM_Archer_Death" :`NewEnumerator3` "/Game/Animations/GreatSword/AM_GreatSword_Death.AM_GreatSword_Death" :`NewEnumerator4` "/Game/Animations/Magic/AM_Magic_Death.AM_Magic_Death" :`NewEnumerator5` "/Game/Animations/OneHanded/AM_SwordAndShield_Death.AM_SwordAndShield_Death" :`NewEnumerator6` "/Game/Animations/Archer/AM_Archer_Death.AM_Archer_Death" :!type "AnimMontage Object Reference")))))

(fn `Get Deflect Animation On Pose`
  (params (Pose :type "/Game/Animations/E_Pose Enum" :default "NewEnumerator0"))
  (returns (`Return Value` :type "AnimMontage Object Reference"))
  (return (select `/Game/Animations/E_Pose` Pose :`NewEnumerator1` "/Game/Animations/Archer/AM_Archer_Block.AM_Archer_Block" :`NewEnumerator2` "/Game/Animations/Fist/AM_Fist_Block.AM_Fist_Block" :`NewEnumerator3` "/Game/Animations/GreatSword/AM_GreatSword_Block.AM_GreatSword_Block" :`NewEnumerator4` "/Game/Animations/Magic/AM_Mage_Block.AM_Mage_Block" :`NewEnumerator5` "/Game/Animations/OneHanded/AM_SwordAndShield_Block_Impact.AM_SwordAndShield_Block_Impact" :`NewEnumerator6` "/Game/Animations/Two-handedAxe/AM_TwoHAxe_Block.AM_TwoHAxe_Block" :!type "AnimMontage Object Reference")))

(fn `Hide Object Widget`
  (`KismetSystemLibrary.K2_ClearTimer` null "Set Object Widget Visible")
  (`SceneComponent.SetVisibility` (`self.Widget`) false true))

(fn `Is NOT Active Montage`
  (returns (ReturnValue :type Boolean))
  (return (not (`AnimInstance.Montage_IsActive` (`SkeletalMeshComponent.GetAnimInstance` (`self.Mesh`)) null))))

(fn `Is NOT Caster?`
  (returns (`Return Value` :type Boolean))
  (locals (`Is Caster` :type Boolean))
  (for _array_element (`self.GetAttachedActors` true)
    (if (or (== _array_element "/Game/Blueprints/Classes/Mage/BP_Class_Mage.BP_Class_Mage") (== _array_element "/Game/Blueprints/Classes/Sorcerer/BP_Class_Sorcerer.BP_Class_Sorcerer"))
      (set `local.Is Caster` true)
      (break)))
  (if (`local.Is Caster`)
    (return false)
    (else
      (return true))))

(fn `Pose Tracker`
  (locals (Weapon :type "/Game/Blueprints/Pickables/Weapons/BP_Weapon_Base Object Reference"))
  ;[1 1 1] If Character Has Weapon, Use Weapon Pose, Otherwise Use Fists Pose
  (for _array_element (`self.Equipment`)
    (bind _asbp_weapon_base (cast `/Game/Blueprints/Pickables/Weapons/BP_Weapon_Base` _array_element))
    (set `local.Weapon` _asbp_weapon_base)
    (break))
  (bind _weapon (`local.Weapon`)
    (:`then`
      (bind _output_get (set `self.Battle Pose` (`/Game/Blueprints/Pickables/Weapons/BP_Weapon_Base.Weapon Pose` _weapon)))
      (set `self.Battle Pose For Caster` _output_get)
      (return))
    (:`else`
      (set `self.Battle Pose` "NewEnumerator2")
      (set `self.Battle Pose For Caster` "NewEnumerator4")
      (return))))

(fn `Remove From Equipment`
  (params (`Item To Remove` :type "/Game/Blueprints/Pickables/BP_PickableItem_Base Object Reference"))
  ;[1 1 1] Remove Item
  (`KismetArrayLibrary.Array_RemoveItem` (`self.Equipment`) `Item To Remove`)
  ;[1 1 1] Check if item is shield, if true, set bool value in character stats
  (if (`|EnumEquality` (`.ItemType_18_4C884E6F4321BC5E70DF60ADCF90B142` (break `/Game/Blueprints/Inventory/ST_Item` (`/Game/Blueprints/Pickables/BP_PickableItem_Base.Item` (`local.Item To Remove`)))) "NewEnumerator3")
    (set `/Game/Blueprints/Stats/AC_CharacterStats.Is Vearing Shield` false (`self.Character Stats`))
    (return)
    (else
      ;[1 1 1] If item is armor (cast is valid, has agility penalty), set bool value in character stats
      (bind _asbp_armor_base (cast `/Game/Blueprints/Pickables/Armor/BP_Armor_Base` (`local.Item To Remove`))
        (:`then`
          (if (> (`/Game/Blueprints/Pickables/Armor/BP_Armor_Base.Penalty To Agility` _asbp_armor_base) 0)
            (set `/Game/Blueprints/Stats/AC_CharacterStats.Is Vearing Armor` false (`self.Character Stats`))
            (return)
            (else
              (return))))
        (:`CastFailed`
          (return))))))

(fn `Set Combat Pose`
  (params (`Is Set` :type Boolean))
  (if `Is Set`
    (if (`self.Is NOT Caster?`)
      (set `self.Current Pose` (`self.Battle Pose`))
      (else
        (set `self.Current Pose` (`self.Battle Pose For Caster`))))
    (return)))

(fn `Set Decal Hovered`
  (`SceneComponent.SetVisibility` (`self.Decal`) true false)
  (`DecalComponent.SetDecalMaterial` (`self.Decal`) (select `/Game/Blueprints/AI/E_AttitudeTowardsPlayer` (`self.Attitude Towards Player`) :`NewEnumerator0` "/Game/Cursor/M_Cursor_NeutralHovered_Decal.M_Cursor_NeutralHovered_Decal" :`NewEnumerator1` "/Game/Cursor/M_Cursor_HostileHovered_Decal.M_Cursor_HostileHovered_Decal" :`NewEnumerator2` "/Game/Cursor/M_Cursor_AlliedHovered_Decal.M_Cursor_AlliedHovered_Decal" :`NewEnumerator3` "/Game/Cursor/M_Cursor_PlayerControlHovered_Decal.M_Cursor_PlayerControlHovered_Decal" :!type "MaterialInterface Object Reference")))

(fn `Set Decal Material LMB`
  (`SceneComponent.SetVisibility` (`self.Decal`) true false)
  (`DecalComponent.SetDecalMaterial` (`self.Decal`) (select `/Game/Blueprints/AI/E_AttitudeTowardsPlayer` (`self.Attitude Towards Player`) :`NewEnumerator0` "/Game/Cursor/M_Cursor_Neutral_Decal.M_Cursor_Neutral_Decal" :`NewEnumerator1` "/Game/Cursor/M_Cursor_Hostile_Decal.M_Cursor_Hostile_Decal" :`NewEnumerator2` "/Game/Cursor/M_Cursor_Allied_Decal.M_Cursor_Allied_Decal" :`NewEnumerator3` "/Game/Cursor/M_Cursor_PlayerControl_Decal.M_Cursor_PlayerControl_Decal" :!type "MaterialInterface Object Reference")))

(fn `Set Object Widget Visible`
  (locals (NewLocalVar_0 :type "Float (double-precision)" :default 1000.0))
  (bind _character_stats (`self.Character Stats`))
  (bind _object_widget (`self.Object Widget`))
  (bind (_returnvalue_roll _returnvalue_pitch _returnvalue_yaw) (`KismetMathLibrary.BreakRotator` (`self.K2_GetActorRotation` (`self.Player Cast`))))
  (`SceneComponent.SetVisibility` (`self.Widget`) true false)
  (`SceneComponent.K2_SetRelativeRotation` (`self.Widget`) (`KismetMathLibrary.MakeRotator` (- _returnvalue_roll 180.0) (- _returnvalue_pitch -125.0) _returnvalue_yaw) false false)
  (set `/Game/HUD/UMG_ObjectName.Object Health` (`KismetMathLibrary.Conv_IntToDouble` (`/Game/Blueprints/Stats/AC_CharacterStats.HP` _character_stats)) _object_widget)
  (set `/Game/HUD/UMG_ObjectName.Object Health Max` (`KismetMathLibrary.Conv_IntToDouble` (`/Game/Blueprints/Stats/AC_CharacterStats.HP Max` _character_stats)) _object_widget)
  (set `/Game/HUD/UMG_ObjectName.Has HP?` true _object_widget)
  (set `/Game/HUD/UMG_ObjectName.Name` (`self.Name`) _object_widget)
  (`SceneComponent.SetRelativeScale3D` (`self.Widget`) (`KismetMathLibrary.Conv_DoubleToVector` (/ (`SpringArmComponent.TargetArmLength` (`/Game/Blueprints/PlayerCamera/BP_PlayerCamera.SpringArm` (`self.Player Cast`))) (`self.Scale Widget Divider`))))
  (return))

(fn `Take Damage`
  (`self.Damage Animation`))

(fn `UserConstructionScript`)