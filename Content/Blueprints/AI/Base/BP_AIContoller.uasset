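; Base AI controller for BP_AICharacter_Base pawns that can start fights from what its pawn perceives.
; BeginPlay caches the player and the controlled character.
; On perception updates, if the pawn and the perceived AI character hold two specific, differing attitudes towards the player and the player is not already fighting, it calls the player's GetAllCharactersToFight with the controlled character.
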(event `self.ReceiveBeginPlay`
  ;[1 1 1] Initial Setup
  (bind _as_player (`/Game/Libraries/BlueprintFunctionLibrary.Cast To Player` 0))
  (set `self.Player Cast` _as_player)
  (bind _asbp_aicharacter_base (cast `/Game/Blueprints/AI/Base/BP_AICharacter_Base` (`self.K2_GetPawn`)))
  (set `self.Controlled Character` _asbp_aicharacter_base))

(event `self.AIPerception.OnTargetPerceptionInfoUpdated`
  (params (UpdateInfo :type "ActorPerceptionUpdateInfo Structure (by ref)"))
  ;[1 1 1] AI Stimulus
  (if (`|EnumEquality` (`/Game/Blueprints/AI/Base/BP_AICharacter_Base.Attitude Towards Player` (`self.Controlled Character`)) "NewEnumerator1")
    (bind _asbp_aicharacter_base (cast `/Game/Blueprints/AI/Base/BP_AICharacter_Base` UpdateInfo_Target))
    (if (`|EnumEquality` (`/Game/Blueprints/AI/Base/BP_AICharacter_Base.Attitude Towards Player` _asbp_aicharacter_base) "NewEnumerator3")
      (if (not (`/Game/Blueprints/PlayerCamera/BP_PlayerCamera.Is In Fight` (`self.Player Cast`)))
        (`/Game/Blueprints/PlayerCamera/BP_PlayerCamera.Get All Characters To Fight` (`self.Player Cast`) (`self.Controlled Character`))))))

(fn `UserConstructionScript`)